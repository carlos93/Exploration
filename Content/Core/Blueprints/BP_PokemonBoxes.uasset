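; Manages the Pokémon storage boxes, a map of box objects that each hold Pokémon by slot index.
; On a new game it creates the default named boxes and fills most slots with random obtainable Pokémon, each given a random ball and recorded in the player's Pokédex.
; Helper functions add to the first empty slot and get, place, remove or swap Pokémon by box and slot, plus rename boxes.
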(event Custom|OnGameStarted
  (bind _returnvalue (Actor|GetActorOfClass "/Game/Core/Blueprints/Player/BP_Player.BP_Player_C"))
  (Variables|Default|SetPlayer _returnvalue)
  (bind _asbp_game_instance (Utilities|Casting|CastToBP_GameInstance (Game|GetGameInstance)))
  (if (Variables|/Game/Core/Blueprints/BP_GameInstance.BP_GameInstance_C|GetIsNewGame _asbp_game_instance)
    (CallFunction|InitDefaultBoxes)))

(fn FillBoxwithRandomPokemons
  (params (BoxId :type Integer))
  (LocalVariables|SetIndex 0)
  (while (< (LocalVariables|GetIndex) (Variables|Default|GetMaxPokemonsPerBox))
    (if (< (Math|Random|RandomFloat) 0.85)
      (bind _output_get (LocalVariables|SetRandomEntry (Math|Random|RandomIntegerinRange 1 251)))
      (bind (_pokemondata _found) (Default|GetPokemon (CallFunction|GetDatabase) _output_get))
      (if (and (not (Variables|/Game/Core/Blueprints/DataAssets/BP_PokemonData.BP_PokemonData_C|GetUnobtainable _pokemondata)) _found)
        (bind _pokemoninfo (CallFunction|CreateRandomPokemonInfo _output_get (Math|Random|RandomIntegerinRange 25 50) true))
        (Default|SetPokedexStatus (Variables|Default|GetPlayer) _output_get (select (Variables|/Game/Core/Blueprints/BP_PokemonInfo.BP_PokemonInfo_C|GetIsShiny _pokemoninfo) "NewEnumerator3" "NewEnumerator2"))
        (bind _itemdata (Default|GetItem (CallFunction|GetDatabase) (Math|Random|RandomIntegerinRange 1 16)))
        (Variables|/Game/Core/Blueprints/BP_PokemonInfo.BP_PokemonInfo_C|SetBall _pokemoninfo (Utilities|ResolveSoftReference _itemdata))
        (Utilities|Map|Add (Variables|/Game/Core/Blueprints/BP_PokemonsBox.BP_PokemonsBox_C|GetBoxPokemons (.Value (Utilities|Map|Find (Variables|Default|GetBoxes) BoxId))) (LocalVariables|GetIndex) _pokemoninfo)
        (Math|Integer|IncrementInt (LocalVariables|GetIndex)))
      (else
        (Math|Integer|IncrementInt (LocalVariables|GetIndex))))))

(fn CreateRandomPokemonInfo
  (params (Entry :type Integer) (Level :type Integer) (CanBeShiny :type Boolean))
  (bind (_pokemondata _found) (Default|GetPokemon (CallFunction|GetDatabase) Entry))
  (if _found
    (return (CallFunction|GeneratePokemonInfo Entry Level _pokemondata CanBeShiny))
    (else
      (Development|PrintString "Pokemon not found"))))

(fn InitDefaultBoxes
  (for _index (range 0 (Variables|Default|GetMaxBoxes))
    (bind _returnvalue (Game|ConstructObjectfromClass "/Game/Core/Blueprints/BP_PokemonsBox.BP_PokemonsBox_C"))
    (Variables|/Game/Core/Blueprints/BP_PokemonsBox.BP_PokemonsBox_C|SetBoxName _returnvalue (Utilities|String|Append "Box " (Utilities|String|ToString(Integer) _index)))
    (Utilities|Map|Add (Variables|Default|GetBoxes) _index _returnvalue)
    (CallFunction|FillBoxwithRandomPokemons _index))
  (Development|PrintString "Boxes created"))

(fn GetFirstEmptySlot
  (bind _boxes (Variables|Default|GetBoxes))
  (bind _keys (Utilities|Map|Keys _boxes))
  (for _array_element _keys
    (for _index (range 0 (Variables|Default|GetMaxPokemonsPerBox))
      (Utilities|IsValid (.Value (Utilities|Map|Find (Variables|/Game/Core/Blueprints/BP_PokemonsBox.BP_PokemonsBox_C|GetBoxPokemons (.Value (Utilities|Map|Find _boxes _array_element))) _index))
        (:Is%20Not%20Valid
          (return _array_element _index)))))
  (return -1 -1))

(fn TrytoAddPokemontoFirstSlotinBox
  (params (PokemonInfo :type BP%20Pokemon%20Info%20Object%20Reference))
  (bind (_box _slot) (CallFunction|GetFirstEmptySlot))
  (if (>= _box 0)
    (Utilities|Map|Add (Variables|/Game/Core/Blueprints/BP_PokemonsBox.BP_PokemonsBox_C|GetBoxPokemons (.Value (Utilities|Map|Find (Variables|Default|GetBoxes) _box))) _slot PokemonInfo))
  (return (>= _box 0)))

(fn GetPokemonInfoinBox
  (params (Box :type Integer) (Slot :type Integer))
  (bind _boxes (Variables|Default|GetBoxes))
  (bind (_value _returnvalue) (Utilities|Map|Find _boxes Box))
  (if _returnvalue
    (return (.Value (Utilities|Map|Find (Variables|/Game/Core/Blueprints/BP_PokemonsBox.BP_PokemonsBox_C|GetBoxPokemons _value) Slot)))
    (else
      (return 0))))

(fn AddPokemontoBox
  (params (Box :type Integer) (Slot :type Integer) (PokemonInfo :type BP%20Pokemon%20Info%20Object%20Reference))
  (Utilities|Map|Add (Variables|/Game/Core/Blueprints/BP_PokemonsBox.BP_PokemonsBox_C|GetBoxPokemons (.Value (Utilities|Map|Find (Variables|Default|GetBoxes) Box))) Slot PokemonInfo))

(fn RemovePokemonfromBox
  (params (Box :type Integer) (Slot :type Integer))
  (Utilities|Map|Remove (Variables|/Game/Core/Blueprints/BP_PokemonsBox.BP_PokemonsBox_C|GetBoxPokemons (.Value (Utilities|Map|Find (Variables|Default|GetBoxes) Box))) Slot))

(fn SwapPokemons
  (params (Box1 :type Integer) (Slot1 :type Integer) (Box2 :type Integer) (Slot2 :type Integer))
  (bind _pokemoninfo (CallFunction|GetPokemonInfoinBox Box1 Slot1))
  (bind _pokemoninfo_2 (CallFunction|GetPokemonInfoinBox Box2 Slot2))
  (bind _output_get (LocalVariables|SetTemp _pokemoninfo))
  (CallFunction|AddPokemontoBox Box1 Slot1 _pokemoninfo_2)
  (CallFunction|AddPokemontoBox Box2 Slot2 _output_get))

(fn SetBoxName
  (params (Box :type Integer) (BoxName :type String))
  (Variables|/Game/Core/Blueprints/BP_PokemonsBox.BP_PokemonsBox_C|SetBoxName (.Value (Utilities|Map|Find (Variables|Default|GetBoxes) Box)) BoxName))