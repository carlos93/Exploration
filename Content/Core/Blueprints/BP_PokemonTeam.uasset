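; Holds the player's Pokémon team as a slot-indexed map, with helpers to add, swap, remove, reorder and find the first one alive.
; On a new game it waits for the database to load, then fills the team with six random obtainable Pokémon, each with a random level, possible shininess and a random item as its ball.
; Generated and added Pokémon update the player's Pokédex status, with shinies marked separately.
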(event Custom|OnDatabaseLoaded
  (bind _database (CallFunction|GetDatabase))
  (bind _asbp_game_instance (Utilities|Casting|CastToBP_GameInstance (Game|GetGameInstance)))
  (if (Variables|/Game/Core/Blueprints/BP_GameInstance.BP_GameInstance_C|GetIsNewGame _asbp_game_instance)
    (bind _result (Default|IsDatabaseLoaded _database))
    (if _result
      (CallFunction|CreateTeam)
      (else
        (EventDispatchers|BindEventtoOnDatabaseLoaded _database (delegate Custom|OnDatabaseLoaded))
        (Development|PrintString "Waiting for database")))))

(event Custom|OnGameStarted
  (params (Player :type BP%20Player%20Object%20Reference))
  (bind _database (CallFunction|GetDatabase))
  (Variables|Default|SetPlayer Player)
  (bind _asbp_game_instance (Utilities|Casting|CastToBP_GameInstance (Game|GetGameInstance)))
  (if (Variables|/Game/Core/Blueprints/BP_GameInstance.BP_GameInstance_C|GetIsNewGame _asbp_game_instance)
    (bind _result (Default|IsDatabaseLoaded _database))
    (if _result
      (CallFunction|CreateTeam)
      (else
        (EventDispatchers|BindEventtoOnDatabaseLoaded _database (delegate Custom|OnDatabaseLoaded))
        (Development|PrintString "Waiting for database")))))

(fn CreatePokemonInfo
  (params (Entry :type Integer) (Level :type Integer) (CanBeShiny :type Boolean))
  (bind (_pokemondata _found) (Default|GetPokemon (CallFunction|GetDatabase) Entry))
  (if _found
    (return (CallFunction|GeneratePokemonInfo Entry Level _pokemondata CanBeShiny))
    (else
      (Development|PrintString "Pokemon not found"))))

(fn CreateTeam
  (Development|PrintString "Starting team creation")
  (Utilities|Map|Clear (Variables|Default|GetTeam))
  (while (< (Utilities|Map|Length (Variables|Default|GetTeam)) 6)
    (bind _output_get (LocalVariables|SetRandomEntry (Math|Random|RandomIntegerinRange 1 251)))
    (bind (_pokemondata _found) (Default|GetPokemon (CallFunction|GetDatabase) _output_get))
    (if (and (not (Variables|/Game/Core/Blueprints/DataAssets/BP_PokemonData.BP_PokemonData_C|GetUnobtainable _pokemondata)) _found)
      (bind _pokemoninfo (CallFunction|CreatePokemonInfo _output_get (Math|Random|RandomIntegerinRange 5 15) true))
      (Default|SetPokedexStatus (Variables|Default|GetPlayer) _output_get (select (Variables|/Game/Core/Blueprints/BP_PokemonInfo.BP_PokemonInfo_C|GetIsShiny _pokemoninfo) "NewEnumerator3" "NewEnumerator2"))
      (bind _itemdata (Default|GetItem (CallFunction|GetDatabase) (Math|Random|RandomIntegerinRange 1 16)))
      (Variables|/Game/Core/Blueprints/BP_PokemonInfo.BP_PokemonInfo_C|SetBall _pokemoninfo (Utilities|ResolveSoftReference _itemdata))
      (Utilities|Map|Add (Variables|Default|GetTeam) (LocalVariables|GetIndex) _pokemoninfo)
      (Math|Integer|IncrementInt (LocalVariables|GetIndex))))
  (Development|PrintString "Team created"))

(fn GetPokemonInfoinSlot
  (params (Slot :type Integer))
  (bind _team (Variables|Default|GetTeam))
  (bind (_value _returnvalue) (Utilities|Map|Find _team Slot))
  (return _value _returnvalue))

(fn GetFirstPokemonAlive
  (bind _values (Utilities|Map|Values (Variables|Default|GetTeam)))
  (for _array_element _values
    (if (> (Variables|/Game/Core/Blueprints/BP_PokemonInfo.BP_PokemonInfo_C|GetCurrentHP _array_element) 0)
      (return _array_element)))
  (return 0))

(fn GetNumPokemonsinTeam
  (return (Utilities|Map|Length (Variables|Default|GetTeam))))

(fn SwapPokemonsinTeam
  (params (From :type Integer) (To :type Integer))
  (bind _team (Variables|Default|GetTeam))
  (bind (_value _returnvalue) (Utilities|Map|Find _team To))
  (bind (_value_2 _returnvalue_2) (Utilities|Map|Find _team From))
  (if (!= From To)
    (if (and _returnvalue_2 _returnvalue)
      (bind _output_get (LocalVariables|SetTemp _value_2))
      (Utilities|Map|Add _team From _value)
      (Utilities|Map|Add _team To _output_get))))

(fn TrytoAddPokemontoTeam
  (params (PokemonInfo :type BP%20Pokemon%20Info%20Object%20Reference))
  (bind _team (Variables|Default|GetTeam))
  (bind _returnvalue (Utilities|Map|Length _team))
  (bind _output_get (LocalVariables|SetTempSuccess (< _returnvalue 6)))
  (if _output_get
    (Utilities|Map|Add _team _returnvalue PokemonInfo)
    (Default|SetPokedexStatus (Variables|Default|GetPlayer) (Variables|/Game/Core/Blueprints/BP_PokemonInfo.BP_PokemonInfo_C|GetEntry PokemonInfo) (select (Variables|/Game/Core/Blueprints/BP_PokemonInfo.BP_PokemonInfo_C|GetIsShiny PokemonInfo) "NewEnumerator3" "NewEnumerator2")))
  (return (LocalVariables|GetTempSuccess)))

(fn SetPokemoninSlot
  (params (Slot :type Integer) (PokemonInfo :type BP%20Pokemon%20Info%20Object%20Reference))
  (bind _team (Variables|Default|GetTeam))
  (Utilities|IsValid PokemonInfo
    (:Is%20Valid
      (Utilities|Map|Add _team Slot PokemonInfo))
    (:Is%20Not%20Valid
      (Utilities|Map|Remove _team Slot))))

(fn RearreangeTeamOrder
  (bind _team (Variables|Default|GetTeam))
  (bind _values (Utilities|Map|Values _team))
  (bind _output_get (LocalVariables|SetTemp _values))
  (Utilities|Map|Clear _team)
  (for _index (range 0 (- (CallFunction|GetMaxPokemonsinTeam) 1))
    (Utilities|IsValid (Utilities|Array|Get(acopy) _output_get _index)
      (:Is%20Valid
        (Utilities|Map|Add _team _index (Utilities|Array|Get(acopy) _output_get _index))))))

(fn RemovePokemonfromSlot
  (params (Slot :type Integer))
  (CallFunction|SetPokemoninSlot Slot))