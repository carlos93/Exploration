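; BP_Inventory stores item stacks as BP_InventoryData objects in a map keyed by item Id.
; On player creation in a new game, it seeds five database items with random amounts, rebinding itself to the database-loaded event if data is not ready.
; AddItem increases an existing stack or constructs a new entry in the given storage map, and HasItem checks whether Storage holds enough of an Id.
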(event Custom|OnPlayerCreated
  (bind _database (CallFunction|GetDatabase))
  (bind _asbp_game_instance (Utilities|Casting|CastToBP_GameInstance (Game|GetGameInstance)))
  (if (Variables|/Game/Core/Blueprints/BP_GameInstance.BP_GameInstance_C|GetIsNewGame _asbp_game_instance)
    (bind _result (Default|IsDatabaseLoaded _database))
    (if _result
      (CallFunction|CreateInventory)
      (else
        (EventDispatchers|BindEventtoOnDatabaseLoaded _database (delegate Custom|OnPlayerCreated))
        (Development|PrintString "Waiting for database")))))

(fn CreateInventory
  (for _index (range 0 4)
    (bind _itemdata (Default|GetItem (CallFunction|GetDatabase) (+ _index 1)))
    (CallFunction|AddItem (Utilities|ResolveSoftReference _itemdata) (Math|Random|RandomIntegerinRange 0 999) (Variables|Default|GetStorage))))

(fn AddItem
  (params (ItemData :type BP%20Item%20Data%20Object%20Reference) (Amount :type Integer) (Storage :type Map%20of%20Integers%20to%20Objects))
  (bind _id (Variables|/Game/Core/Blueprints/DataAssets/BP_BaseData.BP_BaseData_C|GetId ItemData))
  (bind (_value _returnvalue) (Utilities|Map|Find Storage _id))
  (if _returnvalue
    (Variables|/Game/Core/Blueprints/BP_InventoryData.BP_InventoryData_C|SetAmount _value (+ (Variables|/Game/Core/Blueprints/BP_InventoryData.BP_InventoryData_C|GetAmount _value) Amount))
    (else
      (bind _returnvalue_2 (Game|ConstructObjectfromClass "/Game/Core/Blueprints/BP_InventoryData.BP_InventoryData_C"))
      (bind _output_get (Variables|/Game/Core/Blueprints/BP_InventoryData.BP_InventoryData_C|SetItemData _returnvalue_2 ItemData))
      (Variables|/Game/Core/Blueprints/BP_InventoryData.BP_InventoryData_C|SetAmount _returnvalue_2 Amount)
      (Utilities|Map|Add Storage (Variables|/Game/Core/Blueprints/DataAssets/BP_BaseData.BP_BaseData_C|GetId _output_get) _returnvalue_2))))

(fn HasItem
  (params (Id :type Integer) (Amount :type Integer))
  (bind _storage (Variables|Default|GetStorage))
  (bind (_value _returnvalue) (Utilities|Map|Find _storage Id))
  (if _returnvalue
    (LocalVariables|SetRes (>= (Variables|/Game/Core/Blueprints/BP_InventoryData.BP_InventoryData_C|GetAmount _value) Amount))
    (else
      (LocalVariables|SetRes false)))
  (return (LocalVariables|GetRes)))