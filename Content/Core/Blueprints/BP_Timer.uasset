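; BP_Timer is a reusable timer with start, pause and clear functions, a finished callback and optional debug logging.
; StartTimer stores the timeout and either unpauses a valid engine timer handle or sets an engine timer targeting ClearTimer.
; A parallel manual count accumulates elapsed time in UpdateTimer, which nothing in this file calls.
; Tick compares that count to the timeout, then clears the timer and calls OnTimerFinished when exceeded.
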(event EventTick
  (params (DeltaSeconds :type Float%20%28single-precision%29))
  (bind _result (CallFunction|IsTimerFinished))
  (if _result
    (CallFunction|ClearTimer)
    (CallFunction|PrintLogifDebugActive "Timer Expired")
    (Default|CallOnTimerFinished)))

(fn ClearTimer
  (Utilities|Time|ClearandInvalidateTimerbyHandle (Variables|Default|GetTimerHandle))
  (Variables|Default|SetTimeout 0.0)
  (Variables|Default|SetElapsedTime 0.0)
  (CallFunction|PrintLogifDebugActive "Timer Cleared"))

(fn PauseTimer
  (bind _timerhandle (Variables|Default|GetTimerHandle))
  (if (Utilities|Time|IsValidTimerHandle _timerhandle)
    (Utilities|Time|PauseTimerbyHandle _timerhandle)
    (CallFunction|PrintLogifDebugActive "Timer Paused")))

(fn StartTimer
  (params (Timeout :type Float%20%28double-precision%29) (Restart :type Boolean))
  (bind _timerhandle (Variables|Default|GetTimerHandle))
  (if (Utilities|Time|IsValidTimerHandle _timerhandle)
    (if Restart
      (Variables|Default|SetTimeout Timeout))
    (Utilities|Time|UnpauseTimerbyHandle _timerhandle)
    (else
      (bind _output_get (Variables|Default|SetTimeout Timeout))
      (Utilities|Time|SetTimerbyFunctionName 0 "ClearTimer" _output_get)))
  (CallFunction|PrintLogifDebugActive "Timer Started"))

(fn UpdateTimer
  (params (DeltaSeconds :type Float%20%28double-precision%29))
  (bind _result (CallFunction|IsRunning))
  (if _result
    (Variables|Default|SetElapsedTime (+ DeltaSeconds (Variables|Default|GetElapsedTime)))))

(fn IsTimerFinished
  (bind _result (CallFunction|IsRunning))
  (if (and _result (> (Variables|Default|GetElapsedTime) (Variables|Default|GetTimeout)))
    _
    (else
      _))
  (return (and _result (> (Variables|Default|GetElapsedTime) (Variables|Default|GetTimeout)))))

(fn IsRunning
  (return (> (Variables|Default|GetTimeout) 0.0)))

(fn PrintLogifDebugActive
  (params (Text :type Text))
  (if (Variables|Default|GetDebug)
    (Development|PrintText Text))
  (return))