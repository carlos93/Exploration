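; Behavior tree task that sends a Pokémon to a random navigable point within a radius of its origin position.
; The navigation query filter is chosen from whether the Pokémon can swim, walk or both.
; Points too far above or below the origin fail the task, as do failed moves.
; Walk speed is raised for distant targets, and success is reported after a short delay.
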(event EventReceiveExecuteAI
  (params (OwnerController :type AI%20Controller%20Object%20Reference) (ControlledPawn :type Pawn%20Object%20Reference))
  (bind _radius (Variables|Default|GetRadius))
  (bind _asbp_pokemon (Utilities|Casting|CastToBP_Pokemon ControlledPawn))
  (if (Class|Pokemon|CanSwim _asbp_pokemon)
    (if (Class|Pokemon|CanWalk _asbp_pokemon)
      (Variables|Default|SetSelectedFilter "/Game/Core/Blueprints/BP_CanWalkAndSwimFilter.BP_CanWalkAndSwimFilter_C")
      (else
        (Variables|Default|SetSelectedFilter "/Game/Core/Blueprints/BP_CanSwimFilter.BP_CanSwimFilter_C")))
    (else
      (if (Class|Pokemon|CanWalk _asbp_pokemon)
        _
        (else
          _))
      (Variables|Default|SetSelectedFilter "/Game/Core/Blueprints/BP_CanWalkFilter.BP_CanWalkFilter_C")))
  (bind _randomlocation (Class|NavigationSystemV1|GetRandomLocationinNavigableRadius (Variables|/Game/Core/Blueprints/BP_Pokemon.BP_Pokemon_C|GetOriginPosition _asbp_pokemon) _radius 0 (Variables|Default|GetSelectedFilter)))
  (if (> (Math|Float|Absolute(Float) (- (.Z (Math|Vector|BreakVector _randomlocation)) (.Z (Math|Vector|BreakVector (Variables|/Game/Core/Blueprints/BP_Pokemon.BP_Pokemon_C|GetOriginPosition _asbp_pokemon))))) 5e+02)
    (AI|BehaviorTree|FinishExecute false :!label _label)
    (else
      (Variables|/Script/Engine.CharacterMovementComponent|SetMaxWalkSpeed (Variables|/Script/Engine.Character|GetCharacterMovement _asbp_pokemon) (Math|Float|SelectFloat 3e+02 1e+02 (> (Math|Vector|VectorLengthXY (- (Transformation|GetActorLocation ControlledPawn) _randomlocation)) (/ _radius 1.3))))
      (AI|AIMoveTo ControlledPawn _randomlocation 0 5.0 false
        (:OnSuccess
          (Utilities|FlowControl|Delay 0.5)
          (AI|BehaviorTree|FinishExecute true))
        (:OnFail
          (goto _label))))))

(event EventReceiveTickAI
  (params (OwnerController :type AI%20Controller%20Object%20Reference) (ControlledPawn :type Pawn%20Object%20Reference) (DeltaSeconds :type Float%20%28single-precision%29)))