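; BP_Route is an overlap-driven route actor that reports when actors enter or leave it to the level's BP_RouteSystem.
; On BeginPlay it finds and caches the route system with GetActorOfClass.
; Begin and end overlaps call OnRouteEnter and OnRouteExit events, which pass the route and overlapping actor to the system, with ForceShow off on entry.
; It applies no actor filtering itself.
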(event Custom|OnRouteEnter
  (params (Actor :type Actor%20Object%20Reference))
  (Default|OnRouteEnter (Variables|Default|GetRouteSystem) self Actor false))

(event Custom|OnRouteExit
  (params (Actor :type Actor%20Object%20Reference))
  (Default|OnRouteExit (Variables|Default|GetRouteSystem) self Actor))

(event EventBeginPlay
  (bind _returnvalue (Actor|GetActorOfClass "/Game/Core/Blueprints/Systems/BP_RouteSystem.BP_RouteSystem_C"))
  (Variables|Default|SetRouteSystem _returnvalue))

(event Collision|EventActorEndOverlap
  (params (OtherActor :type Actor%20Object%20Reference))
  (CallFunction|OnRouteExit OtherActor))

(event Collision|EventActorBeginOverlap
  (params (OtherActor :type Actor%20Object%20Reference))
  (CallFunction|OnRouteEnter OtherActor))

(fn ConstructionScript)