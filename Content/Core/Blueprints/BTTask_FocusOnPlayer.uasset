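; Behavior tree task that stops a BP_Pokemon and turns it to face its TargetActor, despite the "Player" name.
; On execute it caches the target's location and scales turn speed by the initial yaw difference, then finishes after a fixed delay.
; Each tick it interpolates rotation toward that cached point at constant speed, writing the per-frame yaw step to RotationSpeed.
; An invalid TargetActor leaves the task without a finish call.
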(event EventReceiveTickAI
  (params (OwnerController :type AI%20Controller%20Object%20Reference) (ControlledPawn :type Pawn%20Object%20Reference) (DeltaSeconds :type Float%20%28single-precision%29))
  (bind _asbp_pokemon (Utilities|Casting|CastToBP_Pokemon ControlledPawn))
  (Variables|/Game/Core/Blueprints/BP_Pokemon.BP_Pokemon_C|SetRotationSpeed _asbp_pokemon (.yaw (Math|Rotator|Delta(Rotator) (Class|KismetMathLibrary|RInterptoConstant (Transformation|GetActorRotation _asbp_pokemon) (Math|Rotator|FindLookatRotation (Transformation|GetActorLocation _asbp_pokemon) (Variables|Default|GetTargetPosition)) DeltaSeconds (Variables|Default|GetLerpSpeed)) (Transformation|GetActorRotation _asbp_pokemon))))
  (Transformation|SetActorRotation _asbp_pokemon (Class|KismetMathLibrary|RInterptoConstant (Transformation|GetActorRotation _asbp_pokemon) (Math|Rotator|FindLookatRotation (Transformation|GetActorLocation _asbp_pokemon) (Variables|Default|GetTargetPosition)) DeltaSeconds (Variables|Default|GetLerpSpeed))))

(event EventReceiveExecuteAI
  (params (OwnerController :type AI%20Controller%20Object%20Reference) (ControlledPawn :type Pawn%20Object%20Reference))
  (AI|Navigation|StopMovement OwnerController)
  (bind _asbp_pokemon (Utilities|Casting|CastToBP_Pokemon ControlledPawn)
    (:then
      (if (Utilities|IsValid (Variables|/Game/Core/Blueprints/BP_Pokemon.BP_Pokemon_C|GetTargetActor _asbp_pokemon))
        (bind _output_get (Variables|Default|SetTargetPosition (Transformation|GetActorLocation (Variables|/Game/Core/Blueprints/BP_Pokemon.BP_Pokemon_C|GetTargetActor _asbp_pokemon))))
        (Variables|Default|SetLerpSpeed (Math|Float|Lerp 5.0 1.8e+02 (/ (Math|Float|Clamp(Float) (Math|Float|Absolute(Float) (.yaw (Math|Rotator|Delta(Rotator) (Transformation|GetActorRotation ControlledPawn) (Math|Rotator|FindLookatRotation (Transformation|GetActorLocation ControlledPawn) _output_get)))) 0.0 1.8e+02) 1.8e+02)))
        (Utilities|FlowControl|Delay 2.0 :!label _label)
        (AI|BehaviorTree|FinishExecute true)))
    (:CastFailed
      (goto _label))))