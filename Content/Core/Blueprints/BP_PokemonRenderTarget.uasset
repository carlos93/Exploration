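; BP_PokemonRenderTarget renders a Pokemon to a texture through a scene capture restricted to its own components.
; ChangePokemon reinitializes it by entry and gender; OnInitialize then updates animations and frames the camera from mesh bounds.
; Camera X scales with the log of the bounding radius, and height depends on move type.
; ToggleRendering assigns or clears the texture target, starting off; BeginPlay also caches light and camera positions.
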(event Custom|ChangePokemon
  (params (Entry :type Integer) (Gender :type EPokemonGender%20Enum :default "NewEnumerator0"))
  (Variables|Default|Set_entry Entry)
  (Class|Pokemon|Initialize Entry Gender))

(event EventBeginPlay
  (bind _lights (Variables|Default|GetLights))
  (CallFunction|ToggleRendering false)
  (Utilities|Array|Add _lights (Variables|Default|GetLight1))
  (Utilities|Array|Add _lights (Variables|Default|GetLight2))
  (Utilities|Array|Add _lights (Variables|Default|GetLight3))
  (Utilities|Array|Add _lights (Variables|Default|GetLight4))
  (for _array_element _lights
    (Utilities|Array|Add (Variables|Default|GetLightsOriginalPosition) (Variables|/Script/Engine.SceneComponent|GetRelativeLocation _array_element)))
  (Variables|Default|SetDatabase (CallFunction|GetDatabase))
  (Variables|Default|SetDefaultCameraLocation (Variables|/Script/Engine.SceneComponent|GetRelativeLocation (Variables|Default|GetSceneCaptureComponent2D)))
  (Rendering|SceneCapture|ShowOnlyActorComponents (Variables|Default|GetSceneCaptureComponent2D) self false))

(event EventOnInitialize
  (bind _mesh (Variables|Character|GetMesh))
  (bind _skeletalmeshasset (Variables|/Script/Engine.SkeletalMeshComponent|GetSkeletalMeshAsset _mesh))
  (bind _returnvalue (StaticMesh|GetBounds _skeletalmeshasset))
  (bind (_origin _boxextent _sphereradius) (Math|BoxSphereBounds|BreakBoxSphereBounds _returnvalue))
  (|CallParentFunction)
  (bind _output_get (Variables|Default|SetCurrentMoveType (Variables|/Game/Core/Blueprints/DataAssets/BP_PokemonData.BP_PokemonData_C|GetPreferredMoveType (Variables|/Game/Core/Blueprints/BP_PokemonInfo.BP_PokemonInfo_C|GetPokemonData (Variables|Default|GetPokemonInfo)))))
  (CallFunction|UpdatePokemonAnimations)
  (CallFunction|UpdateonInteractAnimations)
  (Development|PrintString (Utilities|String|ToString(Vector) _origin) true true "(R=0.000000,G=1.000000,B=0.197451,A=1.000000)" 2e+01 "OBounds")
  (Development|PrintString (Utilities|String|ToString(Vector) _boxextent) true true "(R=0.000000,G=1.000000,B=0.197451,A=1.000000)" 2e+01 "BoxBounds")
  (Development|PrintString (Utilities|String|ToString(Float) _sphereradius) true true "(R=0.000000,G=1.000000,B=0.197451,A=1.000000)" 2e+01 "SphereBounds")
  (Transformation|SetRelativeLocation (Variables|Default|GetSceneCaptureComponent2D) (Math|Vector|MakeVector (- (* (Math|Float|Loge _sphereradius) 2.1e+02) 3.5e+02) 0.0 (- (.Z (Math|Vector|BreakVector _boxextent)) (Utilities|Select :Index _output_get :Walk 5.0 :Swim 5.0 :Fly 75.0))) false false))

(fn ConstructionScript
  (|CallParentFunction))

(fn ToggleRendering
  (params (Enable :type Boolean))
  (bind _scenecapturecomponent2d (Variables|Default|GetSceneCaptureComponent2D))
  (if Enable
    (Variables|/Script/Engine.SceneCaptureComponent2D|SetTextureTarget _scenecapturecomponent2d (Variables|Default|GetTexture%20Target))
    (else
      (Variables|/Script/Engine.SceneCaptureComponent2D|SetTextureTarget _scenecapturecomponent2d 0))))

(fn OnStartFlying)

(fn OnEndFlying)