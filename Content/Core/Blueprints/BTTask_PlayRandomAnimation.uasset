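; Behavior tree task that, by random chance, plays an animation on a BP_Pokemon controlled by AI.
; An IsAttack flag selects between the reach-player animation and the stop-move animation.
; Only the attack branch reports success; the stop-move branch, a failed roll and a failed cast all finish as failure.
; The task finishes right after triggering the animation, with no wait for playback to end.
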(event EventReceiveExecuteAI
  (params (OwnerController :type AI%20Controller%20Object%20Reference) (ControlledPawn :type Pawn%20Object%20Reference))
  (if (<= (Math|Random|RandomFloat) (Variables|Default|GetChance))
    (bind _asbp_pokemon (Utilities|Casting|CastToBP_Pokemon ControlledPawn)
      (:then
        (if (Variables|Default|GetIsAttack)
          (Default|PlayonReachPlayerAnim _asbp_pokemon)
          (AI|BehaviorTree|FinishExecute true)
          (else
            (Default|PlayonStopMoveAnim _asbp_pokemon)
            (AI|BehaviorTree|FinishExecute false :!label _label))))
      (:CastFailed
        (goto _label)))
    (else
      (goto _label))))