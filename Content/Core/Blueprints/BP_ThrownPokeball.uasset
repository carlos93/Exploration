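; Thrown Pokéball actor that flies to a target, opens, then closes as the target shrinks, presumably for a capture sequence.
; A timeline blends position toward the target's mesh with a scaled offset and spins the ball.
; Timeline event tracks toggle the open state, spawn a shockwave and trigger the shrink.
; A second timeline rolls the root left or right for bumps; the closed event is an empty stub.
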(event Custom|ThrowToTarget
  (params (Origin :type Transform) (Target :type BP%20Pokemon%20Object%20Reference))
  (bind _mesh (Variables|/Script/Engine.Character|GetMesh Target))
  (bind (_direction _progress _location _rotation) (Timeline|MoveToTarget PlayFromStart)
    (:Update
      (Transformation|SetActorLocation (+ (* _location (Variables|Default|GetMaxLocationDisplacement)) (Math|Vector|Lerp(Vector) (.Location (Math|Transform|BreakTransform Origin)) (Transformation|GetWorldLocation _mesh) _progress)) false false)
      (Transformation|SetWorldRotation (Variables|Character|GetMesh) (Math|Rotator|MakeRotator (.x (* _rotation 3.6e+02)) (.y (* _rotation 3.6e+02)) (.z (* _rotation 3.6e+02))) false false))
    (:Finished
      (Transformation|SetWorldRotation (Variables|Character|GetMesh) (Transformation|GetWorldRotation _mesh) false false))
    (:OnTargetReached
      (Variables|Default|SetIsOpen true)
      (Niagara|SpawnSystematLocation "/Game/Core/Effects/NS_Shockwave.NS_Shockwave" (Transformation|GetActorLocation)))
    (:OnPokeballClose
      (Default|Shrink Target)
      (Variables|Default|SetIsOpen false))))

(event Custom|PlayBump
  (params (ToLeft :type Boolean))
  (bind _defaultsceneroot (Variables|Default|GetDefaultSceneRoot))
  (Variables|Default|SetInitialRotation (Transformation|GetWorldRotation _defaultsceneroot))
  (bind _rotation (Timeline|RotateBump PlayFromStart)
    (:Update
      (Transformation|SetWorldRotation _defaultsceneroot (Math|Rotator|MakeRotator (+ (.Roll (Math|Rotator|BreakRotator (Variables|Default|GetInitialRotation))) (Math|Float|SelectFloat (Math|Float|Lerp 0.0 (Variables|Default|GetAngleToRotate) _rotation) (* (Math|Float|Lerp 0.0 (Variables|Default|GetAngleToRotate) _rotation) -1.0) ToLeft)) (.Pitch (Math|Rotator|BreakRotator (Variables|Default|GetInitialRotation))) (.Yaw (Math|Rotator|BreakRotator (Variables|Default|GetInitialRotation)))) false false))))

(event EventBeginPlay)

(event Collision|EventActorBeginOverlap
  (params (OtherActor :type Actor%20Object%20Reference)))

(event EventTick
  (params (DeltaSeconds :type Float%20%28single-precision%29)))

(event EventEventPokeballClosed)

(fn ConstructionScript)