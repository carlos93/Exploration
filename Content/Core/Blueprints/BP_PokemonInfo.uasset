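; BP_PokemonInfo holds data for a Pokémon, including stats, moves and held item, and exposes query functions over it.
; GetMaxHP looks up the HP entry in the Stats map and falls back to zero when it is missing.
; HasMove scans the Moves map values for a matching move Id, and HasItemEquipped reports whether HeldItem is valid.
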(fn GetMaxHP
  (bind _stats (Variables|Default|GetStats))
  (bind (_value _returnvalue) (Utilities|Map|Find _stats "HP"))
  (if _returnvalue
    (return _value)
    (else
      (return 0))))

(fn HasMove
  (params (MoveData :type BP%20Move%20Data%20Object%20Reference))
  (Utilities|IsValid MoveData
    (:Is%20Valid
      (bind _values (Utilities|Map|Values (Variables|Default|GetMoves)))
      (for _array_element _values
        (if (== (Variables|/Game/Core/Blueprints/DataAssets/BP_BaseData.BP_BaseData_C|GetId _array_element) (Variables|/Game/Core/Blueprints/DataAssets/BP_BaseData.BP_BaseData_C|GetId MoveData))
          (return true))))
    (:Is%20Not%20Valid
      _))
  (return false))

(fn HasItemEquipped
  (return (Utilities|IsValid (Variables|Default|GetHeldItem))))