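; Dialog system actor that reveals a line of text one character at a time, typewriter style.
; ShowText stores the line and dialog box; Tick advances CurrentText while that box is visible.
; An accumulated-time remainder keeps character pacing independent of frame rate.
; Reaching the end calls OnLineFinished once; ForceLineFinished jumps the index to the end to trigger it early.
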(event Custom|ShowText
  (params (Text :type String) (DialogBox :type WB%20Base%20Dialog%20Box%20Object%20Reference))
  (Variables|Default|SetCurrentUI DialogBox)
  (Variables|Default|SetIsLineFinished false)
  (CallFunction|SetTexttoDisplay Text))

(event Custom|ForceLineFinished
  (Variables|Default|SetCharacterIndex (Utilities|String|Len (Variables|Default|GetTextToDisplay)))
  (CallFunction|ShowNextCharacter 0.0))

(event Collision|EventActorBeginOverlap
  (params (OtherActor :type Actor%20Object%20Reference)))

(event EventTick
  (params (DeltaSeconds :type Float%20%28single-precision%29))
  (bind _currentui (Variables|Default|GetCurrentUI))
  (Utilities|IsValid _currentui
    (:Is%20Valid
      (if (Widget|IsVisible _currentui)
        (CallFunction|ShowNextCharacter DeltaSeconds)))))

(event EventBeginPlay)

(fn ConstructionScript)

(fn ShowNextCharacter
  (params (DeltaTime :type Float%20%28double-precision%29))
  (bind _characterindex (Variables|Default|GetCharacterIndex))
  (if (> (Utilities|String|Len (Variables|Default|GetTextToDisplay)) (Variables|Default|GetCharacterIndex))
    (Variables|Default|SetAccumulatedDeltaTimeCharacters (.Remainder (Math|Float|Division(WholeandRemainder) (+ DeltaTime (Variables|Default|GetAccumulatedDeltaTimeCharacters)) (Variables|Default|GetTimeBetweenCharacters))))
    (bind _result (Math|Integer|DecrementInt (.ReturnValue (Math|Float|Division(WholeandRemainder) (+ DeltaTime (Variables|Default|GetAccumulatedDeltaTimeCharacters)) (Variables|Default|GetTimeBetweenCharacters))))
      (:%20%20
        (for _index (range 0 _result)
          (Math|Integer|IncrementInt _characterindex
            (:%20%20
              (Variables|Default|SetCurrentText (Utilities|String|GetSubstring (Variables|Default|GetTextToDisplay) 0 _characterindex)))))))
    (elif (not (Variables|Default|GetIsLineFinished))
      (Variables|Default|SetIsLineFinished true)
      (Default|CallOnLineFinished))))

(fn SetTexttoDisplay
  (params (Text :type String))
  (Variables|Default|SetTextToDisplay Text)
  (Variables|Default|SetCharacterIndex 0))

(fn EventonTextFinished)

(fn Reset
  (Variables|Default|SetCurrentText "")
  (Variables|Default|SetCharacterIndex 0))