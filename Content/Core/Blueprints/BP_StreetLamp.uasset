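; Street lamp actor that switches itself on at night and off during the day.
; Each tick it reads the day progress from the DayNightSubsystem and treats the start and end of the cycle as night.
; Only when that night state changes does it set the SpotLight intensity in candelas and the lamp material's EmissiveStrength parameter to match.
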(event EventBeginPlay)

(event Collision|EventActorBeginOverlap
  (params (OtherActor :type Actor%20Object%20Reference)))

(event EventTick
  (params (DeltaSeconds :type Float%20%28single-precision%29))
  (bind _returnvalue (Subsystems|GetDayNightSubsystem))
  (bind _spotlight (Variables|Default|GetSpotLight))
  (bind __daydonepercentage (Variables|/Script/Exploration.DayNightSubsystem|Get_dayDonePercentage _returnvalue))
  (bind _returnvalue_2 (< __daydonepercentage 0.2))
  (bind _returnvalue_3 (> __daydonepercentage 0.8))
  (bind _returnvalue_4 (or _returnvalue_2 _returnvalue_3))
  (if (!= (Variables|Default|GetOldValue) _returnvalue_4)
    (Variables|Default|SetOldValue _returnvalue_4)
    (Class|LocalLightComponent|SetIntensityUnits _spotlight "Candelas")
    (Rendering|Components|Light|SetIntensity _spotlight (Math|Float|SelectFloat 8.0 0.0 _returnvalue_4))
    (Rendering|Material|SetScalarParameterValueonMaterials (Variables|Default|GetLamp) "EmissiveStrength" (Math|Float|SelectFloat 3.0 0.0 _returnvalue_4))))

(fn ConstructionScript)