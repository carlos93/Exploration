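; BP_Pokeball is an interactable item pickup that shows a dialog for its item when the player interacts with it.
; Interaction focus toggles an outline by switching the mesh's custom depth stencil value.
; StartInteract has BP_Player parse and display the text, with ClosePokeball as the callback that hides the dialog and clears the open flag.
; A separate EventPokeballClosed destroys the actor, but nothing in this graph calls it.
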(event Custom|EventPokeballClosed
  (Actor|DestroyActor))

(event Custom|ClosePokeball
  (bind _returnvalue (Actor|GetActorOfClass "/Game/Core/Blueprints/Player/BP_Player.BP_Player_C"))
  (Default|EventHideDialogBox _returnvalue)
  (Variables|Default|SetIsOpen false))

(event EventBeginPlay)

(event Collision|EventActorBeginOverlap
  (params (OtherActor :type Actor%20Object%20Reference)))

(event EventTick
  (params (DeltaSeconds :type Float%20%28single-precision%29)))

(event EventCanInteract
  (CallFunction|ToggleOutline true))

(event EventStopInteract
  (CallFunction|ToggleOutline false))

(event EventStartInteract
  (params (Actor :type Actor%20Object%20Reference))
  (if (not (Variables|Default|GetIsOpen))
    (bind _asbp_player (Utilities|Casting|CastToBP_Player Actor))
    (bind _result (Default|ParseDialogText _asbp_player (Utilities|String|ToString(Text) (Variables|Default|GetTextToShow)) (Variables|Default|GetItemData)))
    (Default|EventShowDialogBox _asbp_player _result true true 0.0 (delegate Custom|ClosePokeball))
    (Variables|Default|SetIsOpen true)))

(fn ConstructionScript)

(fn ToggleOutline
  (params (Enable :type Boolean))
  (Rendering|SetCustomDepthStencilValue (Variables|Default|GetMesh) (Math|Integer|SelectInt 2 3 Enable)))