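; BP_SaveGame converts the player's Pokémon team and inventory between runtime objects and save-friendly structs.
; Serialize functions walk each map and flatten Pokémon and inventory objects into structs, storing balls, held items and inventory items as IDs.
; Deserialize functions rebuild the maps with newly constructed BP_PokemonInfo and BP_InventoryData objects, resolving those IDs back to item data through the Database.
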(fn SerializeTeam
  (params (Team :type Map%20of%20Integers%20to%20Objects))
  (bind _keys (Utilities|Map|Keys Team))
  (for _array_element _keys
    (if (.ReturnValue (Utilities|Map|Find Team _array_element))
      (bind _output (CallFunction|SerializePokemonInfo (.Value (Utilities|Map|Find Team _array_element))))
      (Utilities|Map|Add (LocalVariables|GetTemp) _array_element _output)))
  (return (LocalVariables|GetTemp)))

(fn SerializePokemonInfo
  (params (PokemonInfo :type BP%20Pokemon%20Info%20Object%20Reference))
  (return (Utilities|Struct|MakeBP_PokemonInfoSaveGame (Variables|/Game/Core/Blueprints/BP_PokemonInfo.BP_PokemonInfo_C|GetName PokemonInfo) (Variables|/Game/Core/Blueprints/BP_PokemonInfo.BP_PokemonInfo_C|GetEntry PokemonInfo) (Variables|/Game/Core/Blueprints/BP_PokemonInfo.BP_PokemonInfo_C|GetLevel PokemonInfo) (Variables|/Game/Core/Blueprints/BP_PokemonInfo.BP_PokemonInfo_C|GetStats PokemonInfo) (Variables|/Game/Core/Blueprints/BP_PokemonInfo.BP_PokemonInfo_C|GetIVs PokemonInfo) (Variables|/Game/Core/Blueprints/BP_PokemonInfo.BP_PokemonInfo_C|GetEVs PokemonInfo) (Variables|/Game/Core/Blueprints/BP_PokemonInfo.BP_PokemonInfo_C|GetMoves PokemonInfo) (Variables|/Game/Core/Blueprints/BP_PokemonInfo.BP_PokemonInfo_C|GetNature PokemonInfo) (Variables|/Game/Core/Blueprints/BP_PokemonInfo.BP_PokemonInfo_C|GetGender PokemonInfo) (Variables|/Game/Core/Blueprints/BP_PokemonInfo.BP_PokemonInfo_C|GetAbility PokemonInfo) (Variables|/Game/Core/Blueprints/BP_PokemonInfo.BP_PokemonInfo_C|GetCurrentHP PokemonInfo) (Variables|/Game/Core/Blueprints/BP_PokemonInfo.BP_PokemonInfo_C|GetCurrentPPs PokemonInfo) (Variables|/Game/Core/Blueprints/BP_PokemonInfo.BP_PokemonInfo_C|GetCurrentExp PokemonInfo) (Variables|/Game/Core/Blueprints/DataAssets/BP_BaseData.BP_BaseData_C|GetId (Variables|/Game/Core/Blueprints/BP_PokemonInfo.BP_PokemonInfo_C|GetBall PokemonInfo)) (Variables|/Game/Core/Blueprints/BP_PokemonInfo.BP_PokemonInfo_C|GetIsShiny PokemonInfo) (Variables|/Game/Core/Blueprints/BP_PokemonInfo.BP_PokemonInfo_C|GetPrimaryStatusCondition PokemonInfo) (Variables|/Game/Core/Blueprints/BP_PokemonInfo.BP_PokemonInfo_C|GetSecondaryStatusCondition PokemonInfo) (Variables|/Game/Core/Blueprints/DataAssets/BP_BaseData.BP_BaseData_C|GetId (Variables|/Game/Core/Blueprints/BP_PokemonInfo.BP_PokemonInfo_C|GetHeldItem PokemonInfo)))))

(fn SerializeInventory
  (params (Inventory :type Map%20of%20Integers%20to%20Objects))
  (bind _keys (Utilities|Map|Keys Inventory))
  (for _array_element _keys
    (if (.ReturnValue (Utilities|Map|Find Inventory _array_element))
      (bind _output (CallFunction|SerializeItem (.Value (Utilities|Map|Find Inventory _array_element))))
      (Utilities|Map|Add (LocalVariables|GetTemp) _array_element _output)))
  (return (LocalVariables|GetTemp)))

(fn SerializeItem
  (params (InventoryData :type BP%20Inventory%20Data%20Object%20Reference))
  (return (Utilities|Struct|MakeBP_ItemSaveGame (Variables|/Game/Core/Blueprints/DataAssets/BP_BaseData.BP_BaseData_C|GetId (Variables|/Game/Core/Blueprints/BP_InventoryData.BP_InventoryData_C|GetItemData InventoryData)) (Variables|/Game/Core/Blueprints/BP_InventoryData.BP_InventoryData_C|GetAmount InventoryData))))

(fn DeserializeTeam
  (params (Input :type Map%20of%20Integers%20to%20Structs))
  (bind _keys (Utilities|Map|Keys Input))
  (for _array_element _keys
    (if (.ReturnValue (Utilities|Map|Find Input _array_element))
      (bind _pokemoninfo (CallFunction|DeserializePokemonInfo (.Value (Utilities|Map|Find Input _array_element))))
      (Utilities|Map|Add (LocalVariables|GetTemp) _array_element _pokemoninfo)))
  (return (LocalVariables|GetTemp)))

(fn DeserializePokemonInfo
  (params (Input :type BP%20Pokemon%20Info%20Save%20Game%20Structure))
  (bind (_name _entry _level _stats _ivs _evs _moves _nature _gender _ability _currenthp _currentpps _currentexp _ballentry _isshiny _primarystatuscondition _secondarystatuscondition _helditem) (Utilities|Struct|BreakBP_PokemonInfoSaveGame Input))
  (bind _database (Variables|Default|GetDatabase))
  (bind _returnvalue (Game|ConstructObjectfromClass "/Game/Core/Blueprints/BP_PokemonInfo.BP_PokemonInfo_C"))
  (Variables|/Game/Core/Blueprints/BP_PokemonInfo.BP_PokemonInfo_C|SetName _returnvalue _name)
  (Variables|/Game/Core/Blueprints/BP_PokemonInfo.BP_PokemonInfo_C|SetEntry _returnvalue _entry)
  (Variables|/Game/Core/Blueprints/BP_PokemonInfo.BP_PokemonInfo_C|SetLevel _returnvalue _level)
  (Variables|/Game/Core/Blueprints/BP_PokemonInfo.BP_PokemonInfo_C|SetStats _returnvalue _stats)
  (Variables|/Game/Core/Blueprints/BP_PokemonInfo.BP_PokemonInfo_C|SetIVs _returnvalue _ivs)
  (Variables|/Game/Core/Blueprints/BP_PokemonInfo.BP_PokemonInfo_C|SetEVs _returnvalue _evs)
  (Variables|/Game/Core/Blueprints/BP_PokemonInfo.BP_PokemonInfo_C|SetMoves _returnvalue _moves)
  (Variables|/Game/Core/Blueprints/BP_PokemonInfo.BP_PokemonInfo_C|SetNature _returnvalue _nature)
  (Variables|/Game/Core/Blueprints/BP_PokemonInfo.BP_PokemonInfo_C|SetGender _returnvalue _gender)
  (Variables|/Game/Core/Blueprints/BP_PokemonInfo.BP_PokemonInfo_C|SetAbility _returnvalue _ability)
  (Variables|/Game/Core/Blueprints/BP_PokemonInfo.BP_PokemonInfo_C|SetCurrentHP _returnvalue _currenthp)
  (Variables|/Game/Core/Blueprints/BP_PokemonInfo.BP_PokemonInfo_C|SetCurrentPPs _returnvalue _currentpps)
  (Variables|/Game/Core/Blueprints/BP_PokemonInfo.BP_PokemonInfo_C|SetCurrentExp _returnvalue _currentexp)
  (bind _itemdata (Default|GetItem _database _ballentry))
  (Variables|/Game/Core/Blueprints/BP_PokemonInfo.BP_PokemonInfo_C|SetBall _returnvalue (Utilities|ResolveSoftReference _itemdata))
  (Variables|/Game/Core/Blueprints/BP_PokemonInfo.BP_PokemonInfo_C|SetIsShiny _returnvalue _isshiny)
  (bind _itemdata_2 (Default|GetItem _database _helditem))
  (Variables|/Game/Core/Blueprints/BP_PokemonInfo.BP_PokemonInfo_C|SetHeldItem _returnvalue (Utilities|ResolveSoftReference _itemdata_2))
  (Variables|/Game/Core/Blueprints/BP_PokemonInfo.BP_PokemonInfo_C|SetPrimaryStatusCondition _returnvalue _primarystatuscondition)
  (Variables|/Game/Core/Blueprints/BP_PokemonInfo.BP_PokemonInfo_C|SetSecondaryStatusCondition _returnvalue _secondarystatuscondition)
  (return _returnvalue))

(fn DeserializeInventory
  (params (Input :type Map%20of%20Integers%20to%20Structs))
  (bind _keys (Utilities|Map|Keys Input))
  (for _array_element _keys
    (if (.ReturnValue (Utilities|Map|Find Input _array_element))
      (bind _inventorydata (CallFunction|DeserializeItem (.Value (Utilities|Map|Find Input _array_element))))
      (Utilities|Map|Add (LocalVariables|GetTemp) _array_element _inventorydata)))
  (return (LocalVariables|GetTemp)))

(fn DeserializeItem
  (params (Input :type BP%20Item%20Save%20Game%20Structure))
  (bind (_entry _amount) (Utilities|Struct|BreakBP_ItemSaveGame Input))
  (bind _returnvalue (Game|ConstructObjectfromClass "/Game/Core/Blueprints/BP_InventoryData.BP_InventoryData_C"))
  (bind _itemdata (Default|GetItem (Variables|Default|GetDatabase) _entry))
  (Variables|/Game/Core/Blueprints/BP_InventoryData.BP_InventoryData_C|SetItemData _returnvalue (Utilities|ResolveSoftReference _itemdata))
  (Variables|/Game/Core/Blueprints/BP_InventoryData.BP_InventoryData_C|SetAmount _returnvalue _amount)
  (return _returnvalue))