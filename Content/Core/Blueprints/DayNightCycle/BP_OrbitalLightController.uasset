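; Orbital light controller that rotates a referenced light actor through the day-night cycle.
; RotateLight offsets the DayNightSubsystem's day-done percentage, wraps it to one cycle, optionally remaps it through ProgressionCurve, then samples RotationCurve as fractions of 360 degrees per axis.
; Tick updates immediately on the first frame, then uses a Delay to throttle updates to BP_ThirdPersonGameMode's OrbitUpdateInterval.
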(event EventBeginPlay)

(event Collision|EventActorBeginOverlap
  (params (OtherActor :type Actor%20Object%20Reference)))

(event EventTick
  (params (DeltaSeconds :type Float%20%28single-precision%29))
  (if (Variables|Default|GetIsFirstTick)
    (Variables|Default|SetIsFirstTick false)
    (else
      (bind _asbp_third_person_game_mode (Utilities|Casting|CastToBP_ThirdPersonGameMode (Game|GetGameMode))
        (:then
          (Utilities|FlowControl|Delay (Variables|/Game/Core/Blueprints/BP_ThirdPersonGameMode.BP_ThirdPersonGameMode_C|GetOrbitUpdateInterval _asbp_third_person_game_mode)))
        (:CastFailed
          _))))
  (CallFunction|RotateLight (Variables|Default|GetLight) (Variables|Default|GetRotationCurve) (Variables|Default|GetProgressionCurve)))

(fn ConstructionScript)

(fn RotateLight
  (params (Light :type Directional%20Light%20Object%20Reference) (RotationCurve :type Curve%20Vector%20Object%20Reference) (ProgressionCurve :type Curve%20Float%20Object%20Reference))
  (bind _returnvalue (Math|Float|MakeLiteralFloat 3.6e+02))
  (bind _returnvalue_2 (Utilities|IsValid ProgressionCurve))
  (bind _returnvalue_3 (Subsystems|GetDayNightSubsystem))
  (bind _offset (Variables|Default|GetOffset))
  (bind __daydonepercentage (Variables|/Script/Exploration.DayNightSubsystem|Get_dayDonePercentage _returnvalue_3))
  (bind _returnvalue_4 (+ _offset __daydonepercentage))
  (bind _remainder (Math|Float|Division(WholeandRemainder) _returnvalue_4 1.0))
  (bind _returnvalue_5 (Math|Curves|GetFloatValue ProgressionCurve _remainder))
  (bind _returnvalue_6 (Math|Float|SelectFloat _returnvalue_5 _remainder _returnvalue_2))
  (bind _returnvalue_7 (Math|Curves|GetVectorValue RotationCurve _returnvalue_6))
  (bind _returnvalue_8 (* _returnvalue_7 _returnvalue))
  (Utilities|IsValid RotationCurve
    (:Is%20Valid
      (Transformation|SetActorRotation Light (Math|Rotator|MakeRotator (.x _returnvalue_8) (.y _returnvalue_8) (.z _returnvalue_8))))))