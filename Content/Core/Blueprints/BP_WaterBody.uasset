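; BP_WaterBody is a water volume that tells overlapping Pokemon and players when they enter or leave water.
; Its Collision component's begin and end overlap events switch swim-capable Pokemon between Swim and Walk move types.
; The same events set or clear IsInWater on BP_Player and print enter and exit debug text.
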(event OnComponentBeginOverlap(Collision)
  (params (OverlappedComponent :type Primitive%20Component%20Object%20Reference) (OtherActor :type Actor%20Object%20Reference) (OtherComp :type Primitive%20Component%20Object%20Reference) (OtherBodyIndex :type Integer) (bFromSweep :type Boolean) (SweepResult :type Hit%20Result%20Structure%20%28by%20ref%29))
  (Development|PrintText "EnterWater")
  (Utilities|FlowControl|Sequence
    (:then_0
      (bind _aspokemon (Utilities|Casting|CastToPokemon OtherActor))
      (if (Class|Pokemon|CanSwim _aspokemon)
        (Variables|/Script/Exploration.Pokemon|Set_currentMoveTypes _aspokemon "Swim")))
    (:then_1
      (bind _asbp_player (Utilities|Casting|CastToBP_Player OtherActor))
      (Variables|/Game/Core/Blueprints/BP_Player.BP_Player_C|SetIsInWater _asbp_player true))))

(event OnComponentEndOverlap(Collision)
  (params (OverlappedComponent :type Primitive%20Component%20Object%20Reference) (OtherActor :type Actor%20Object%20Reference) (OtherComp :type Primitive%20Component%20Object%20Reference) (OtherBodyIndex :type Integer))
  (Development|PrintText "ExitWater")
  (Utilities|FlowControl|Sequence
    (:then_0
      (bind _aspokemon (Utilities|Casting|CastToPokemon OtherActor))
      (if (Class|Pokemon|CanSwim _aspokemon)
        (Variables|/Script/Exploration.Pokemon|Set_currentMoveTypes _aspokemon "Walk")))
    (:then_1
      (bind _asbp_player (Utilities|Casting|CastToBP_Player OtherActor))
      (Variables|/Game/Core/Blueprints/BP_Player.BP_Player_C|SetIsInWater _asbp_player false))))

(event EventBeginPlay)

(event EventTick
  (params (DeltaSeconds :type Float%20%28single-precision%29)))

(fn ConstructionScript)