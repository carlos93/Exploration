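; Level-placed spawner that periodically populates its radius with wild Pokémon, up to a maximum count.
; A Tick-driven timer runs once the database and game are ready, pausing when the player is far away.
; Each spawn is a chance-weighted pick filtered by time of day, placed on navmesh using walk/swim query filters.
; It then receives behaviour and movement bitmasks plus generated level and info from the database.
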(event OnTimerFinished(SpawnTimer)
  (if (< (Variables|Data|GetNumSpawnedPokemons) (Variables|Data|GetMaxSpawnedPokemons))
    (CallFunction|SpawnPokemon))
  (Default|StartTimer (Variables|Default|GetSpawnTimer) (Variables|Data|GetMinTimeBetweenSpawns) true))

(event Custom|On%20Pokemon%20Destroyed
  (Math|Integer|DecrementInt (Variables|Data|GetNumSpawnedPokemons)))

(event EventBeginPlay
  (Variables|Default|SetDatabase (CallFunction|GetDatabase))
  (Default|StartTimer (Variables|Default|GetSpawnTimer) (Math|Random|RandomFloatinRange (Variables|Data|GetMinTimeBetweenSpawns) (Variables|Data|GetMaxTimeBetweenSpawns)) true))

(event EventTick
  (params (DeltaSeconds :type Float%20%28single-precision%29))
  (bind _spawntimer (Variables|Default|GetSpawnTimer))
  (bind _spawntimer_2 (Variables|Default|GetSpawnTimer))
  (bind _asbp_third_person_game_mode (Utilities|Casting|CastToBP_ThirdPersonGameMode (Game|GetGameMode)))
  (bind _result (Default|IsDatabaseLoaded (Variables|Default|GetDatabase)))
  (if (and _result (Variables|/Game/Core/Blueprints/BP_ThirdPersonGameMode.BP_ThirdPersonGameMode_C|GetIsGameStarted _asbp_third_person_game_mode))
    (if (> (Transformation|GetDistanceTo (Game|GetPlayerCharacter 0)) (+ (Variables|Data|GetDeactivateDistance) (Variables|Data|GetMaxSpawnRadius)))
      (Default|ClearTimer _spawntimer)
      (else
        (bind _result_2 (Default|IsRunning _spawntimer))
        (if _result_2
          (Default|UpdateTimer _spawntimer_2 DeltaSeconds)
          (else
            (Default|StartTimer _spawntimer_2 (Variables|Data|GetMinTimeBetweenSpawns) true)))))))

(fn ConstructionScript
  (Components|Sphere|SetSphereRadius (Variables|Default|GetSphere) (Variables|Data|GetMaxSpawnRadius) true))

(fn SpawnPokemon
  (bind (_res _valid) (CallFunction|GetRandomWeighted (Variables|Data|GetSpawnerData) (Class|DayNightSubsystem|GetCurrentTimeDay (Subsystems|GetDayNightSubsystem))))
  (if _valid
    (for _array_element (.behaviourtype _res)
      (LocalVariables|SetBehaviourMask (+ (Math|Float|Truncate (Math|Float|Power 2.0 (Math|Conversions|ToFloat(Integer) (Math|Conversions|ToInteger(Byte) _array_element)))) (LocalVariables|GetBehaviourMask))))
    (for _array_element_2 (.allowedmovetypes _res)
      (LocalVariables|SetMoveMask (+ (Math|Conversions|ToInteger(Byte) _array_element_2) (LocalVariables|GetMoveMask))))
    (bind _pokemondata (Default|GetPokemon (Variables|Default|GetDatabase) (.entry _res)))
    (bind (_randomlocation _returnvalue) (Class|NavigationSystemV1|GetRandomLocationinNavigableRadius (Transformation|GetActorLocation) (Variables|Data|GetMaxSpawnRadius) 0 (select (and (not (Variables|/Game/Core/Blueprints/DataAssets/BP_PokemonData.BP_PokemonData_C|GetCanWalkInWater _pokemondata)) (and (!= (Class|KismetMathLibrary|AndIntInt (LocalVariables|GetMoveMask) (Math|Conversions|ToInteger(Byte) (Utilities|Enum|LiteralenumEPokemonMoveType "Walk"))) 0) (!= (Class|KismetMathLibrary|AndIntInt (LocalVariables|GetMoveMask) (Math|Conversions|ToInteger(Byte) (Utilities|Enum|LiteralenumEPokemonMoveType "Swim"))) 0))) "/Game/Core/Blueprints/BP_CanWalkAndSwimFilter.BP_CanWalkAndSwimFilter_C" (select (and (not (Variables|/Game/Core/Blueprints/DataAssets/BP_PokemonData.BP_PokemonData_C|GetCanWalkInWater _pokemondata)) (!= (Class|KismetMathLibrary|AndIntInt (LocalVariables|GetMoveMask) (Math|Conversions|ToInteger(Byte) (Utilities|Enum|LiteralenumEPokemonMoveType "Swim"))) 0)) "/Game/Core/Blueprints/BP_CanSwimFilter.BP_CanSwimFilter_C" "/Game/Core/Blueprints/BP_CanWalkFilter.BP_CanWalkFilter_C"))))
    (if _returnvalue
      (bind _returnvalue_2 (Game|SpawnActorfromClass "/Game/Core/Blueprints/BP_Pokemon.BP_Pokemon_C" (Math|Transform|MakeTransform _randomlocation (Math|Rotator|MakeRotator 0.0 0.0 (.yaw (Math|Random|RandomRotator false))) (Math|Conversions|ToVector(Float) (Math|Random|RandomFloatinRange 1.2 1.4))) "Undefined" "MultiplyWithRoot" 0 0))
      (Variables|/Script/Exploration.Pokemon|Set_entry _returnvalue_2 (.entry _res))
      (Variables|/Game/Core/Blueprints/BP_Pokemon.BP_Pokemon_C|SetSpawner _returnvalue_2 self)
      (Variables|/Script/Exploration.Pokemon|Set_allowedMoveTypes _returnvalue_2 (Class|KismetMathLibrary|OrIntInt (LocalVariables|GetMoveMask) (|BitmaskLiteral)))
      (Variables|/Game/Core/Blueprints/BP_Pokemon.BP_Pokemon_C|SetBehaviourType _returnvalue_2 (|BitmaskLiteral (LocalVariables|GetBehaviourMask)))
      (bind _res_2 (Default|HasBehaviour _returnvalue_2 "NewEnumerator5"))
      (Variables|/Game/Core/Blueprints/BP_Pokemon.BP_Pokemon_C|SetIsPlayingSpecialAnimation _returnvalue_2 _res_2)
      (Variables|/Game/Core/Blueprints/BP_Pokemon.BP_Pokemon_C|SetCurrentMoveType _returnvalue_2 (select (> (Utilities|Array|Length (Collision|GetOverlappingActors _returnvalue_2 "/Game/Core/Blueprints/BP_WaterBody.BP_WaterBody_C" :!class /Script/Engine.Actor)) 0) (Utilities|Enum|LiteralenumEPokemonMoveType "Swim") (Utilities|Enum|LiteralenumEPokemonMoveType (Variables|/Script/Exploration.Pokemon|Get_defaultMoveType _returnvalue_2))))
      (Math|Integer|IncrementInt (Variables|Data|GetNumSpawnedPokemons)
        (:%20%20
          (bind _output_get (Variables|/Game/Core/Blueprints/BP_Pokemon.BP_Pokemon_C|SetPokemonInfo _returnvalue_2 (CallFunction|GeneratePokemonInfo (.entry _res) (Math|Random|RandomIntegerinRange (.levelmin _res) (.levelmax _res)) _pokemondata true)))
          (Variables|/Game/Core/Blueprints/BP_PokemonInfo.BP_PokemonInfo_C|SetPokemonData _output_get _pokemondata)
          (Default|EventSpawn _returnvalue_2 (select (Variables|/Game/Core/Blueprints/DataAssets/BP_PokemonData.BP_PokemonData_C|GetHasGenderDifferences _pokemondata) (Variables|/Game/Core/Blueprints/BP_PokemonInfo.BP_PokemonInfo_C|GetGender _output_get) "NewEnumerator0")))))))

(fn GetRandomWeighted
  (params (Array :type Array%20of%20BP%20Pokemon%20Spawner%20Data%20Structures) (DayTime :type EDayTime%20Enum :default "Day"))
  (for _array_element Array
    (if (Utilities|Array|ContainsItem (.alloweddaytimes _array_element) DayTime)
      (LocalVariables|SetTotalWeight (+ (.chance _array_element) (LocalVariables|GetTotalWeight)))))
  (LocalVariables|SetRandomSelected (Math|Random|RandomFloatinRange 0.0 (LocalVariables|GetTotalWeight)))
  (for _array_element_2 Array
    (if (Utilities|Array|ContainsItem (.AllowedDayTimes (Utilities|Struct|BreakBP_PokemonSpawnerData _array_element_2)) DayTime)
      (bind _output_get (LocalVariables|SetCursor (+ (.Chance (Utilities|Struct|BreakBP_PokemonSpawnerData _array_element_2)) (LocalVariables|GetCursor))))
      (if (>= _output_get (LocalVariables|GetRandomSelected))
        (return _array_element_2 true))))
  (Development|PrintText "Error in algorithm" true true "(R=1.000000,G=0.017480,B=0.000000,A=1.000000)")
  (return "" false))