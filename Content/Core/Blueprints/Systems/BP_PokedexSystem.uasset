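; Pokédex system that records each Pokémon entry's status in a map, with queries for seen and captured progress.
; Status writes only ever raise an entry's level by comparing enum integer values, and missing entries read as the default status.
; Seen and captured checks share an "at or above" comparison, so higher statuses also satisfy lower ones.
; The total count includes only entries whose status exactly matches the requested one.
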(event EventBeginPlay)

(event Collision|EventActorBeginOverlap
  (params (OtherActor :type Actor%20Object%20Reference)))

(event EventTick
  (params (DeltaSeconds :type Float%20%28single-precision%29)))

(fn ConstructionScript)

(fn GetPokedexStatus
  (params (Entry :type Integer))
  (bind _pokedexstatusmap (Variables|Default|GetPokedexStatusMap))
  (bind (_value _returnvalue) (Utilities|Map|Find _pokedexstatusmap Entry))
  (if _returnvalue
    (return _value)
    (else
      (return "NewEnumerator0"))))

(fn SetPokedexStatus
  (params (Entry :type Integer) (PokedexStatus :type EPokedexStatus%20Enum :default "NewEnumerator0"))
  (bind _pokedexstatusmap (Variables|Default|GetPokedexStatusMap))
  (bind (_value _returnvalue) (Utilities|Map|Find _pokedexstatusmap Entry))
  (if _returnvalue
    (if (> (Math|Conversions|ToInteger(Byte) PokedexStatus) (Math|Conversions|ToInteger(Byte) _value))
      (Utilities|Map|Add _pokedexstatusmap Entry PokedexStatus :!label _label))
    (else
      (goto _label))))

(fn HasPokemonPokedexStatusorHigher
  (params (Entry :type Integer) (PokedexStatus :type EPokedexStatus%20Enum :default "NewEnumerator0"))
  (bind _pokedexstatusmap (Variables|Default|GetPokedexStatusMap))
  (bind (_value _returnvalue) (Utilities|Map|Find _pokedexstatusmap Entry))
  (if _returnvalue
    (return (>= (Math|Conversions|ToInteger(Byte) _value) (Math|Conversions|ToInteger(Byte) PokedexStatus)))
    (else
      (return false))))

(fn IsPokemonCaptured
  (params (Entry :type Integer))
  (return (CallFunction|HasPokemonPokedexStatusorHigher Entry "NewEnumerator2")))

(fn IsPokemonSeen
  (params (Entry :type Integer))
  (return (CallFunction|HasPokemonPokedexStatusorHigher Entry "NewEnumerator1")))

(fn GetTotalPokemonwithStatus
  (params (PokedexStatus :type EPokedexStatus%20Enum :default "NewEnumerator0"))
  (bind _pokedexstatusmap (Variables|Default|GetPokedexStatusMap))
  (bind _keys (Utilities|Map|Keys _pokedexstatusmap))
  (for _array_element _keys
    (if (and (.ReturnValue (Utilities|Map|Find _pokedexstatusmap _array_element)) (Utilities|Enum|Equal(Enum) PokedexStatus (.Value (Utilities|Map|Find _pokedexstatusmap _array_element))))
      (Math|Integer|IncrementInt (LocalVariables|GetTotal))))
  (return (LocalVariables|GetTotal)))