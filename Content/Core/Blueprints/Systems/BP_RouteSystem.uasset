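; BP_RouteSystem tracks the player's current route and drives its music and location-name display.
; Entering a differently named or forced route crossfades to that route's music if different, shows its name on the player's WB_RouteInfo widget and starts a display timer.
; Exiting a route re-enters the parent BP_Route it is attached to, supporting nested routes.
; ToggleMusic pauses or resumes the current track.
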(event Custom|OnRouteEnter
  (params (Route :type BP%20Route%20Object%20Reference) (Actor :type Actor%20Object%20Reference) (ForceShow :type Boolean))
  (bind _currentmusiccomponent (Variables|Default|GetCurrentMusicComponent))
  (bind _routeinfo (Variables|/Game/Core/Blueprints/BP_Route.BP_Route_C|GetRouteInfo Route))
  (Utilities|IsValid Route
    (:Is%20Valid
      (Utilities|IsValid (Variables|Default|GetCurrentRoute)
        (:Is%20Valid
          (if (not (and (not ForceShow) (Utilities|Enum|Equal(Enum) (.name _routeinfo) (.name (Variables|/Game/Core/Blueprints/BP_Route.BP_Route_C|GetRouteInfo (Variables|Default|GetCurrentRoute))))))
            (Utilities|FlowControl|Sequence :!label _label
              (:then_0
                (Development|PrintString (Utilities|String|Append "Entered " (Utilities|String|ToString(Text) (.name _routeinfo)))))
              (:then_1
                (Utilities|IsValid _currentmusiccomponent
                  (:Is%20Valid
                    (if (!= (.music _routeinfo) (Variables|/Script/Engine.AudioComponent|GetSound _currentmusiccomponent))
                      (Audio|Components|Audio|FadeOut _currentmusiccomponent (Variables|Default|GetFadeDuration) 0.0 "Linear" :!class /Script/Engine.AudioComponent)
                      (CallFunction|PlayRouteMusic (.music _routeinfo) :!label _label_2)))
                  (:Is%20Not%20Valid
                    (goto _label_2))))
              (:then_2
                (bind _asbp_player (Utilities|Casting|CastToBP_Player Actor))
                (bind _result (Default|GetWidgetfromEnum _asbp_player "NewEnumerator2"))
                (bind _aswb_route_info (Utilities|Casting|CastToWB_RouteInfo _result))
                (Default|ShowLocationName _aswb_route_info (.name _routeinfo))
                (Default|StartTimer (Variables|/Game/Core/Blueprints/Player/BP_Player.BP_Player_C|GetShowLocationTimer _asbp_player) 5.0 false)
                (Variables|Default|SetCurrentRoute Route)))))
        (:Is%20Not%20Valid
          (goto _label))))))

(event Custom|OnRouteExit
  (params (Route :type BP%20Route%20Object%20Reference) (Actor :type Actor%20Object%20Reference))
  (bind _returnvalue (Actor|GetAttachParentActor Route))
  (Utilities|FlowControl|Sequence
    (:then_0
      (Development|PrintText (Utilities|Text|ToText(String) (Utilities|String|Append "Exited " (Utilities|String|ToString(Text) (.name (Variables|/Game/Core/Blueprints/BP_Route.BP_Route_C|GetRouteInfo Route)))))))
    (:then_1
      (Utilities|IsValid _returnvalue
        (:Is%20Valid
          (bind _asbp_route (Utilities|Casting|CastToBP_Route _returnvalue))
          (Default|OnRouteEnter _asbp_route Actor))))))

(event Custom|ToggleMusic
  (params (Enable :type Boolean))
  (bind _currentmusiccomponent (Variables|Default|GetCurrentMusicComponent))
  (Utilities|IsValid _currentmusiccomponent
    (:Is%20Valid
      (Class|AudioComponent|SetPaused _currentmusiccomponent (not Enable)))))

(event Custom|PlayRouteMusic
  (params (Music :type Sound%20Wave%20Object%20Reference))
  (bind _returnvalue (Audio|SpawnSound2D Music 1.0 1.0 0.0 0))
  (Audio|Components|Audio|FadeIn _returnvalue (Variables|Default|GetFadeDuration) 1.0 0.0 "Linear" :!class /Script/Engine.AudioComponent)
  (Variables|Default|SetCurrentMusicComponent _returnvalue))

(fn ConstructionScript)