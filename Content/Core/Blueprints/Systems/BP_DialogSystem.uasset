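; Dialog system actor that reveals lines of text character by character, typewriter style, for a dialog box widget.
; ShowText stores the line, widget and callback; Tick advances CurrentText at a fixed character interval while the widget is visible.
; A finished line fires OnLineFinished, then after any required input and an extra delay calls and unbinds the callback.
; ForceLineFinished jumps to the line's end, and OnActionSelected clears the input wait.
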(event Custom|OnActionSelected
  (Variables|Default|SetShouldWaitForInput false))

(event Custom|ForceLineFinished
  (Variables|Default|SetCharacterIndex (Utilities|String|Len (Variables|Default|GetTextToDisplay)))
  (CallFunction|ShowNextCharacter 0.0))

(event Collision|EventActorBeginOverlap
  (params (OtherActor :type Actor%20Object%20Reference)))

(event EventTick
  (params (DeltaSeconds :type Float%20%28single-precision%29))
  (bind _currentui (Variables|Default|GetCurrentUI))
  (Utilities|IsValid _currentui
    (:Is%20Valid
      (if (Widget|IsVisible _currentui)
        (CallFunction|ShowNextCharacter DeltaSeconds)
        (if (Math|Boolean|ANDBoolean (Variables|Default|GetShouldTriggerCallback) (Variables|Default|GetIsLineFinished) (not (Variables|Default|GetShouldWaitForInput)))
          (Utilities|FlowControl|Delay (Variables|Default|GetExtraDelay))
          (Variables|Default|SetShouldTriggerCallback false)
          (Default|CallLineFinishedCallback)
          (EventDispatchers|UnbindallEventsfromLineFinishedCallback))))))

(event EventBeginPlay)

(fn ConstructionScript)

(fn ShowNextCharacter
  (params (DeltaTime :type Float%20%28double-precision%29))
  (bind _characterindex (Variables|Default|GetCharacterIndex))
  (if (> (Utilities|String|Len (Variables|Default|GetTextToDisplay)) (Variables|Default|GetCharacterIndex))
    (Variables|Default|SetAccumulatedDeltaTimeCharacters (.Remainder (Math|Float|Division(WholeandRemainder) (+ DeltaTime (Variables|Default|GetAccumulatedDeltaTimeCharacters)) (Variables|Default|GetTimeBetweenCharacters))))
    (bind _result (Math|Integer|DecrementInt (.ReturnValue (Math|Float|Division(WholeandRemainder) (+ DeltaTime (Variables|Default|GetAccumulatedDeltaTimeCharacters)) (Variables|Default|GetTimeBetweenCharacters))))
      (:%20%20
        (for _index (range 0 _result)
          (Math|Integer|IncrementInt _characterindex
            (:%20%20
              (Variables|Default|SetCurrentText (Utilities|String|GetSubstring (Variables|Default|GetTextToDisplay) 0 _characterindex)))))))
    (elif (not (Variables|Default|GetIsLineFinished))
      (Variables|Default|SetIsLineFinished true)
      (Default|CallOnLineFinished)
      (Variables|Default|SetShouldTriggerCallback true))))

(fn SetTexttoDisplay
  (params (Text :type String))
  (Variables|Default|SetCharacterIndex 0)
  (Variables|Default|SetTextToDisplay Text))

(fn EventonTextFinished)

(fn Reset
  (Variables|Default|SetCurrentText "")
  (Variables|Default|SetCharacterIndex 0))

(fn ShowText
  (params (Text :type String) (DialogBox :type WB%20Base%20Dialog%20Box%20Object%20Reference) (ShouldWaitForInput :type Boolean) (ExtraDelay :type Float%20%28double-precision%29) (Callback :type Delegate%20%28by%20ref%29))
  (EventDispatchers|BindEventtoLineFinishedCallback Callback)
  (Variables|Default|SetCurrentUI DialogBox)
  (Variables|Default|SetIsLineFinished false)
  (Variables|Default|SetShouldTriggerCallback false)
  (CallFunction|SetTexttoDisplay Text)
  (Variables|Default|SetShouldWaitForInput ShouldWaitForInput)
  (Variables|Default|SetExtraDelay ExtraDelay)
  (Development|PrintString Text false))