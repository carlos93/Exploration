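; Central Pokémon game database that async-loads data, icons and cry assets at startup and serves them through ID-based getters.
; InitLoading starts seven parallel primary-asset loads that fill maps for Pokémon, moves, items, abilities, icons and cries, then fires CallOnDatabaseLoaded once all flags are set.
; Pokémon data nests by ID, regional form and form via wrapper objects, while icon and cry keys are parsed from asset names.
; Model loading exists but is disconnected.
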(event Custom|OnPokemonAssetsLoaded
  (params (Assets :type Array%20of%20Object%20Object%20References))
  (for _array_element Assets
    (bind _asbp_pokemon_data (Utilities|Casting|CastToBP_PokemonData _array_element))
    (CallFunction|AddPokemonDatatoMap _asbp_pokemon_data))
  (Variables|Default|SetIsPokemonDatabaseLoaded true)
  (Development|PrintString (Utilities|String|Append "Loaded " (Utilities|String|ToString(Integer) (Utilities|Map|Length (Variables|Default|GetPokemons))) " pokemons"))
  (bind _result (CallFunction|IsDatabaseLoaded))
  (if _result
    (Default|CallOnDatabaseLoaded)))

(event Custom|OnAbilityAssetsLoaded
  (params (Assets :type Array%20of%20Object%20Object%20References))
  (for _array_element Assets
    (bind _asbp_ability_data (Utilities|Casting|CastToBP_AbilityData _array_element))
    (Utilities|Map|Add (Variables|Default|GetAbilities) (Variables|/Game/Core/Blueprints/DataAssets/BP_AbilityData.BP_AbilityData_C|GetId _asbp_ability_data) (Utilities|ResolveSoftReference _asbp_ability_data)))
  (Development|PrintString (Utilities|String|Append "Loaded " (Utilities|String|ToString(Integer) (Utilities|Map|Length (Variables|Default|GetAbilities))) " abilities"))
  (Variables|Default|SetIsAbilitiesDatabaseLoaded true)
  (bind _result (CallFunction|IsDatabaseLoaded))
  (if _result
    (Default|CallOnDatabaseLoaded)))

(event Custom|OnMoveAssetsLoaded
  (params (Assets :type Array%20of%20Object%20Object%20References))
  (for _array_element Assets
    (bind _asbp_move_data (Utilities|Casting|CastToBP_MoveData _array_element))
    (Utilities|Map|Add (Variables|Default|GetMoves) (Variables|/Game/Core/Blueprints/DataAssets/BP_PokemonData.BP_PokemonData_C|GetId _asbp_move_data) (Utilities|ResolveSoftReference _asbp_move_data)))
  (Development|PrintString (Utilities|String|Append "Loaded " (Utilities|String|ToString(Integer) (Utilities|Map|Length (Variables|Default|GetMoves))) " moves"))
  (Variables|Default|SetIsMovesDatabaseLoaded true)
  (bind _result (CallFunction|IsDatabaseLoaded))
  (if _result
    (Default|CallOnDatabaseLoaded)))

(event Custom|OnItemAssetsLoaded
  (params (Assets :type Array%20of%20Object%20Object%20References))
  (for _array_element Assets
    (bind _asbp_item_data (Utilities|Casting|CastToBP_ItemData _array_element))
    (Utilities|Map|Add (Variables|Default|GetItems) (Variables|/Game/Core/Blueprints/DataAssets/BP_AbilityData.BP_AbilityData_C|GetId _asbp_item_data) (Utilities|ResolveSoftReference _asbp_item_data)))
  (Development|PrintString (Utilities|String|Append "Loaded " (Utilities|String|ToString(Integer) (Utilities|Map|Length (Variables|Default|GetItems))) " items"))
  (Variables|Default|SetIsItemsDatabaseLoaded true)
  (bind _result (CallFunction|IsDatabaseLoaded))
  (if _result
    (Default|CallOnDatabaseLoaded)))

(event Custom|OnModelsLoaded
  (params (Assets :type Array%20of%20Object%20Object%20References))
  (for _array_element Assets
    (bind _asskeletal_mesh (Utilities|Casting|CastToSkeletalMesh _array_element))
    (Utilities|Map|Add (Variables|Default|GetModels) (Math|Conversions|ToInteger(Byte) (Utilities|String|Right (Utilities|GetObjectName _array_element) 4)) _asskeletal_mesh))
  (Development|PrintString (Utilities|String|Append "Loaded " (Utilities|String|ToString(Integer) (Utilities|Map|Length (Variables|Default|GetModels))) " models"))
  (Variables|Default|SetIsModelsDatabaseLoaded true)
  (bind _result (CallFunction|IsDatabaseLoaded))
  (if _result
    (Default|CallOnDatabaseLoaded)))

(event Custom|OnIconAssetsLoaded
  (params (Assets :type Array%20of%20Object%20Object%20References))
  (for _array_element Assets
    (bind _astexture_2d (Utilities|Casting|CastToTexture2D _array_element))
    (if (Utilities|String|Contains (Utilities|GetObjectName _array_element) "upscaled")
      (Utilities|Map|Add (Variables|Default|GetPokemonIconsBig) (Math|Conversions|ToInteger(Byte) (.RightS (Utilities|String|Split (Utilities|GetObjectName _array_element) "-" "IgnoreCase" "FromEnd"))) _astexture_2d)
      (else
        (Utilities|Map|Add (Variables|Default|GetPokemonIcons) (Math|Conversions|ToInteger(Byte) (Utilities|String|Right (Utilities|String|Left (Utilities|GetObjectName _array_element) 6) 4)) _astexture_2d))))
  (Development|PrintString (Utilities|String|Append "Loaded " (Utilities|String|ToString(Integer) (Utilities|Map|Length (Variables|Default|GetPokemonIcons))) " icons and " (Utilities|String|ToString(Integer) (Utilities|Map|Length (Variables|Default|GetPokemonIconsBig))) " big icons"))
  (Variables|Default|SetIsIconsDatabaseLoaded true)
  (bind _result (CallFunction|IsDatabaseLoaded))
  (if _result
    (Default|CallOnDatabaseLoaded)))

(event Custom|OnCriesAssetsLoaded
  (params (Assets :type Array%20of%20Object%20Object%20References))
  (for _array_element Assets
    (bind _assound_wave (Utilities|Casting|CastToSoundWave _array_element))
    (Utilities|Map|Add (Variables|Default|GetPokemonCries) (Math|Conversions|ToInteger(Byte) (Utilities|GetObjectName _array_element)) _assound_wave))
  (Development|PrintString (Utilities|String|Append "Loaded " (Utilities|String|ToString(Integer) (Utilities|Map|Length (Variables|Default|GetPokemonCries))) " cries"))
  (Variables|Default|SetIsCriesDatabaseLoaded true)
  (bind _result (CallFunction|IsDatabaseLoaded))
  (if _result
    (Default|CallOnDatabaseLoaded)))

(event Custom|InitLoading
  (Utilities|FlowControl|Sequence
    (:then_0
      (bind _outprimaryassetidlist (Class|KismetSystemLibrary|GetPrimaryAssetIdList "BP_PokemonData_C"))
      (bind _loaded (|AsyncLoadPrimaryAssetList _outprimaryassetidlist)
        (:Completed
          (CallFunction|OnPokemonAssetsLoaded _loaded))))
    (:then_1
      (bind _outprimaryassetidlist_2 (Class|KismetSystemLibrary|GetPrimaryAssetIdList "BP_MoveData_C"))
      (bind _loaded_2 (|AsyncLoadPrimaryAssetList _outprimaryassetidlist_2)
        (:Completed
          (CallFunction|OnMoveAssetsLoaded _loaded_2))))
    (:then_2
      (bind _outprimaryassetidlist_3 (Class|KismetSystemLibrary|GetPrimaryAssetIdList "BP_ItemData_C"))
      (bind _loaded_3 (|AsyncLoadPrimaryAssetList _outprimaryassetidlist_3)
        (:Completed
          (CallFunction|OnItemAssetsLoaded _loaded_3))))
    (:then_3
      (bind _outprimaryassetidlist_4 (Class|KismetSystemLibrary|GetPrimaryAssetIdList "BP_AbilityData_C"))
      (bind _loaded_4 (|AsyncLoadPrimaryAssetList _outprimaryassetidlist_4)
        (:Completed
          (CallFunction|OnAbilityAssetsLoaded _loaded_4))))
    (:then_4
      (bind _outprimaryassetidlist_5 (Class|KismetSystemLibrary|GetPrimaryAssetIdList "Icons"))
      (bind _loaded_5 (|AsyncLoadPrimaryAssetList _outprimaryassetidlist_5)
        (:Completed
          (CallFunction|OnIconAssetsLoaded _loaded_5))))
    (:then_5
      (bind _outprimaryassetidlist_6 (Class|KismetSystemLibrary|GetPrimaryAssetIdList "Cry"))
      (bind _loaded_6 (|AsyncLoadPrimaryAssetList _outprimaryassetidlist_6)
        (:Completed
          (CallFunction|OnCriesAssetsLoaded _loaded_6))))
    (:then_6
      (bind _outprimaryassetidlist_7 (Class|KismetSystemLibrary|GetPrimaryAssetIdList "ItemIcons"))
      (bind _loaded_7 (|AsyncLoadPrimaryAssetList _outprimaryassetidlist_7)
        (:Completed
          (CallFunction|OnItemIconsAssetsLoaded _loaded_7))))))

(event Custom|OnItemIconsAssetsLoaded
  (params (Assets :type Array%20of%20Object%20Object%20References))
  (for _array_element Assets
    (bind _astexture_2d (Utilities|Casting|CastToTexture2D _array_element))
    (Utilities|Map|Add (Variables|Default|GetItemIcons) (Math|Conversions|ToInteger(Byte) (Utilities|GetObjectName _array_element)) _astexture_2d))
  (Development|PrintString (Utilities|String|Append "Loaded " (Utilities|String|ToString(Integer) (Utilities|Map|Length (Variables|Default|GetItemIcons))) " item sprites"))
  (Variables|Default|SetIsItemIconsDatabaseLoaded true)
  (bind _result (CallFunction|IsDatabaseLoaded))
  (if _result
    (Default|CallOnDatabaseLoaded)))

(fn ConstructionScript)

(fn IsDatabaseLoaded
  (return (Math|Boolean|ANDBoolean (Variables|Default|GetIsPokemonDatabaseLoaded) (Variables|Default|GetIsMovesDatabaseLoaded) (Variables|Default|GetIsAbilitiesDatabaseLoaded) (Variables|Default|GetIsItemsDatabaseLoaded) (Variables|Default|GetIsIconsDatabaseLoaded) (Variables|Default|GetIsCriesDatabaseLoaded) (Variables|Default|GetIsItemIconsDatabaseLoaded))))

(fn GetAbility
  (params (Id :type Integer))
  (bind _abilities (Variables|Default|GetAbilities))
  (bind (_value _returnvalue) (Utilities|Map|Find _abilities Id))
  (return _value _returnvalue))

(fn GetPokemon
  (params (Id :type Integer) (RegionalForm :type EPokemonRegionalFormType%20Enum :default "None") (Form :type Integer))
  (bind _returnvalue (< Form 10))
  (bind _pokemons (Variables|Default|GetPokemons))
  (bind _returnvalue_2 (Math|Integer|SelectInt 0 Form _returnvalue))
  (bind (_value _returnvalue_3) (Utilities|Map|Find _pokemons Id))
  (bind _map (Variables|/Game/Core/Blueprints/BP_PokemonDataRegionalFormsMap.BP_PokemonDataRegionalFormsMap_C|GetMap _value))
  (bind (_value_2 _returnvalue_4) (Utilities|Map|Find _map RegionalForm))
  (bind _map_2 (Variables|/Game/Core/Blueprints/BP_PokemonDataFormsMap.BP_PokemonDataFormsMap_C|GetMap _value_2))
  (bind (_value_3 _returnvalue_5) (Utilities|Map|Find _map_2 _returnvalue_2))
  (if _returnvalue_3
    (if _returnvalue_4
      (return _value_3 _returnvalue_5))))

(fn GetMove
  (params (Id :type Integer))
  (bind _moves (Variables|Default|GetMoves))
  (bind (_value _returnvalue) (Utilities|Map|Find _moves Id))
  (return (Utilities|ResolveSoftReference _value) _returnvalue))

(fn GetPokemonIcon
  (params (Id :type Integer))
  (bind _pokemonicons (Variables|Default|GetPokemonIcons))
  (bind (_value _returnvalue) (Utilities|Map|Find _pokemonicons Id))
  (return _value _returnvalue))

(fn GetPokemonCry
  (params (Id :type Integer))
  (bind _pokemoncries (Variables|Default|GetPokemonCries))
  (bind (_value _returnvalue) (Utilities|Map|Find _pokemoncries Id))
  (return _value _returnvalue))

(fn GetItemIcon
  (params (Id :type Integer))
  (bind _itemicons (Variables|Default|GetItemIcons))
  (bind (_value _returnvalue) (Utilities|Map|Find _itemicons Id))
  (return _value _returnvalue))

(fn GetItem
  (params (Id :type Integer))
  (bind _items (Variables|Default|GetItems))
  (bind (_value _returnvalue) (Utilities|Map|Find _items Id))
  (return _value _returnvalue))

(fn GetPokemonBigIcon
  (params (Id :type Integer))
  (bind _pokemoniconsbig (Variables|Default|GetPokemonIconsBig))
  (bind (_value _returnvalue) (Utilities|Map|Find _pokemoniconsbig Id))
  (return _value _returnvalue))

(fn AddPokemonDatatoMap
  (params (PokemonData :type BP%20Pokemon%20Data%20Object%20Reference%20%28by%20ref%29))
  (bind _id (Variables|/Game/Core/Blueprints/DataAssets/BP_BaseData.BP_BaseData_C|GetId PokemonData))
  (bind _regionalform (Variables|/Game/Core/Blueprints/DataAssets/BP_PokemonData.BP_PokemonData_C|GetRegionalForm PokemonData))
  (bind _pokemons (Variables|Default|GetPokemons))
  (bind (_value _returnvalue) (Utilities|Map|Find _pokemons _id))
  (bind _map (Variables|/Game/Core/Blueprints/BP_PokemonDataRegionalFormsMap.BP_PokemonDataRegionalFormsMap_C|GetMap _value))
  (bind (_value_2 _returnvalue_2) (Utilities|Map|Find _map _regionalform))
  (if _returnvalue
    _
    (else
      (bind _returnvalue_3 (Game|ConstructObjectfromClass "/Game/Core/Blueprints/BP_PokemonDataRegionalFormsMap.BP_PokemonDataRegionalFormsMap_C"))
      (Utilities|Map|Add _pokemons _id _returnvalue_3)))
  (if _returnvalue_2
    _
    (else
      (bind _returnvalue_4 (Game|ConstructObjectfromClass "/Game/Core/Blueprints/BP_PokemonDataFormsMap.BP_PokemonDataFormsMap_C"))
      (Utilities|Map|Add _map _regionalform _returnvalue_4)))
  (Utilities|Map|Add (Variables|/Game/Core/Blueprints/BP_PokemonDataFormsMap.BP_PokemonDataFormsMap_C|GetMap _value_2) (Variables|/Game/Core/Blueprints/DataAssets/BP_PokemonData.BP_PokemonData_C|GetForm PokemonData) PokemonData))

(fn GetPokemonForms
  (params (Id :type Integer) (RegionalForm :type EPokemonRegionalFormType%20Enum :default "None"))
  (bind _pokemons (Variables|Default|GetPokemons))
  (bind (_value _returnvalue) (Utilities|Map|Find _pokemons Id))
  (bind _map (Variables|/Game/Core/Blueprints/BP_PokemonDataRegionalFormsMap.BP_PokemonDataRegionalFormsMap_C|GetMap _value))
  (bind (_value_2 _returnvalue_2) (Utilities|Map|Find _map RegionalForm))
  (if _returnvalue
    (if _returnvalue_2
      (return _value_2))))

(fn GetPokemonRegionalForms
  (params (Id :type Integer))
  (return (.Value (Utilities|Map|Find (Variables|Default|GetPokemons) Id))))

(fn HasMultipleForms
  (params (Id :type Integer))
  (bind _forms (CallFunction|GetPokemonRegionalForms Id))
  (bind _keys (Utilities|Map|Keys (Variables|/Game/Core/Blueprints/BP_PokemonDataRegionalFormsMap.BP_PokemonDataRegionalFormsMap_C|GetMap _forms)))
  (if (> (Utilities|Array|Length _keys) 1)
    (return true)
    (else
      (for _array_element _keys
        (bind _forms_2 (CallFunction|GetPokemonForms Id _array_element))
        (bind _values (Utilities|Map|Values (Variables|/Game/Core/Blueprints/BP_PokemonDataFormsMap.BP_PokemonDataFormsMap_C|GetMap _forms_2)))
        (if (> (Utilities|Array|Length _values) 1)
          (LocalVariables|SetCount 0)
          (for _array_element_2 _values
            (if (not (or (Variables|/Game/Core/Blueprints/DataAssets/BP_PokemonData.BP_PokemonData_C|GetIsGigamax _array_element_2) (Variables|/Game/Core/Blueprints/DataAssets/BP_PokemonData.BP_PokemonData_C|GetIsMega _array_element_2)))
              (Math|Integer|IncrementInt (LocalVariables|GetCount))))
          (return (> (LocalVariables|GetCount) 1))
          (else
            (return false))))
      (return false))))

(fn HasMultipleRegionalForms
  (params (Id :type Integer))
  (bind _forms (CallFunction|GetPokemonRegionalForms Id))
  (return (Utilities|Map|IsNotEmpty (Variables|/Game/Core/Blueprints/BP_PokemonDataRegionalFormsMap.BP_PokemonDataRegionalFormsMap_C|GetMap _forms))))