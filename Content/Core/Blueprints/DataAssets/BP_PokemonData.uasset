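; BP_PokemonData is a Pokémon data Blueprint that answers whether that Pokémon can learn a given move.
; CanLearnMove scans the Moves array for an entry whose move Id matches the supplied move data and whose learn method matches the requested one.
; A learn method of None acts as a wildcard, so any entry with a matching Id qualifies.
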(fn CanLearnMove
  (params (MoveData :type BP%20Move%20Data%20Object%20Reference) (MoveLearnMethod :type EPokemonMoveLearnMethod%20Enum :default "None"))
  (bind _array_element (Utilities|Array|ForEachLoopwithBreak (Variables|Default|GetMoves))
    (:LoopBody
      (if (or (Utilities|Enum|Equal(Enum) MoveLearnMethod "None") (Utilities|Enum|Equal(Enum) (.MoveLearnMethod (Utilities|Struct|BreakBP_MoveLearnData _array_element)) MoveLearnMethod))
        (if (== (Variables|/Game/Core/Blueprints/DataAssets/BP_BaseData.BP_BaseData_C|GetId (.Move (Utilities|Struct|BreakBP_MoveLearnData _array_element))) (Variables|/Game/Core/Blueprints/DataAssets/BP_BaseData.BP_BaseData_C|GetId MoveData))
          (return true))))
    (:Completed
      (return false))))