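; BP_ItemData is an item data asset that decides whether the item can be used by a given Pokémon.
; IsUsableBy returns true when the Pokémon's entry matches an Id in the UsableBy list.
; Otherwise, items with a valid TmMove defer to the Pokémon data's CanLearnMove check for the Machine learn method, and all others return false.
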(fn IsUsableby
  (params (PokemonInfo :type BP%20Pokemon%20Info%20Object%20Reference))
  (bind _tmmove (Variables|Default|GetTmMove))
  (for _array_element (Variables|Default|GetUsableBy)
    (if (== (Variables|/Game/Core/Blueprints/DataAssets/BP_BaseData.BP_BaseData_C|GetId _array_element) (Variables|/Game/Core/Blueprints/BP_PokemonInfo.BP_PokemonInfo_C|GetEntry PokemonInfo))
      (return true)))
  (Utilities|IsValid _tmmove
    (:Is%20Valid
      (return (Default|CanLearnMove (Variables|/Game/Core/Blueprints/BP_PokemonInfo.BP_PokemonInfo_C|GetPokemonData PokemonInfo) _tmmove "Machine")))
    (:Is%20Not%20Valid
      (return false))))