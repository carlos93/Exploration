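; BP_NPC is an interactable NPC whose skeletal mesh and idle, walk and run animations are chosen by its NpcEntry enum.
; It async-loads these assets by enum-derived names on BeginPlay, while the construction script swaps the mesh through the asset registry when the entry changes.
; Interaction turns it toward the player and shows dialog text, then restores its orientation afterward.
; An outline highlight toggles through custom depth stencil values.
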(event Custom|LoadAnimations
  (bind _npcentry (Variables|NPC|GetNpcEntry))
  (bind _returnvalue (Utilities|String|EnumtoString _npcentry))
  (Utilities|Map|Clear (Variables|Default|GetAnimations))
  (bind _loaded (|AsyncLoadPrimaryAssetList (Utilities|Array|MakeArray (Utilities|Struct|MakePrimaryAssetId "NpcAnimations" (Utilities|String|StringToName (Utilities|String|Append _returnvalue "_idle"))) (Utilities|Struct|MakePrimaryAssetId "NpcAnimations" (Utilities|String|StringToName (Utilities|String|Append _returnvalue "_walk"))) (Utilities|Struct|MakePrimaryAssetId "NpcAnimations" (Utilities|String|StringToName (Utilities|String|Append _returnvalue "_run")))))
    (:Completed
      (for (_array_element _array_index) _loaded
        (bind _asanim_sequence (Utilities|Casting|CastToAnimSequence _array_element))
        (Utilities|Map|Add (Variables|Default|GetAnimations) (Utilities|Enum|ByteToEnumENpcAnimations (Math|Conversions|ToByte(Integer) _array_index)) _asanim_sequence)))))

(event Custom|LoadModel
  (bind _loaded (|AsyncLoadPrimaryAsset (Utilities|Struct|MakePrimaryAssetId "NPCModels" (Utilities|String|StringToName (Utilities|String|EnumtoString (Variables|NPC|GetNpcEntry)))))
    (:then
      (bind _asskeletal_mesh (Utilities|Casting|CastToSkeletalMesh _loaded))
      (Components|SkeletalMesh|SetSkeletalMeshAsset (Variables|Character|GetMesh) _asskeletal_mesh))))

(event Custom|HideText
  (bind _returnvalue (Actor|GetActorOfClass "/Game/Core/Blueprints/Player/BP_Player.BP_Player_C"))
  (Default|HideOpenWorldDialogBox _returnvalue)
  (Variables|Default|SetIsInteractionActive false)
  (Transformation|SetActorRotation (Variables|Default|GetOriginalOrientation)))

(event EventBeginPlay
  (CallFunction|LoadModel)
  (CallFunction|LoadAnimations)
  (Variables|Default|SetOriginalOrientation (Transformation|GetWorldRotation (Variables|Collision|GetCapsuleComponent))))

(event Collision|EventActorBeginOverlap
  (params (OtherActor :type Actor%20Object%20Reference)))

(event EventTick
  (params (DeltaSeconds :type Float%20%28single-precision%29)))

(event EventCanInteract
  (CallFunction|ToggleOutline true))

(event EventStopInteract
  (CallFunction|ToggleOutline false))

(event EventStartInteract
  (params (Actor :type Actor%20Object%20Reference))
  (bind _returnvalue (Transformation|GetActorRotation))
  (bind (_roll _pitch) (Math|Rotator|BreakRotator _returnvalue))
  (if (not (Variables|Default|GetIsInteractionActive))
    (bind _asbp_player (Utilities|Casting|CastToBP_Player Actor))
    (bind _dialogbox (Default|GetDialogPanel _asbp_player false))
    (Default|ShowMultipleText _dialogbox (Variables|NPC|GetInteractTexts) (delegate Custom|HideText))
    (Variables|Default|SetIsInteractionActive true)
    (Transformation|SetActorRotation (Math|Rotator|MakeRotator _roll _pitch (.Yaw (Math|Rotator|BreakRotator (Math|Rotator|FindLookatRotation (Transformation|GetActorLocation) (Transformation|GetActorLocation _asbp_player))))))))

(fn ConstructionScript
  (bind _npcentry (Variables|NPC|GetNpcEntry))
  (bind _returnvalue (Utilities|String|EnumtoString _npcentry))
  (if (not (Utilities|Enum|Equal(Enum) (Variables|NPC|GetNpcEntry) (Variables|Default|GetOldNpcEntry)))
    (Variables|Default|SetOldNpcEntry (Variables|NPC|GetNpcEntry))
    (bind _returnvalue_2 (Class|AssetRegistry|GetAssetbyObjectPath (Class|AssetRegistryHelpers|GetAssetRegistry) (Utilities|MakeSoftObjectPath (Utilities|String|Append "/Game/Core/NPCs/" _returnvalue "/" _returnvalue "." _returnvalue)) false true))
    (bind _asskeletal_mesh (Utilities|Casting|CastToSkeletalMesh (Class|AssetRegistryHelpers|GetAsset _returnvalue_2)))
    (Components|SkeletalMesh|SetSkeletalMeshAsset (Variables|Character|GetMesh) _asskeletal_mesh)))

(fn ToggleOutline
  (params (Show :type Boolean))
  (Rendering|SetCustomDepthStencilValue (Variables|Character|GetMesh) (Math|Integer|SelectInt 2 1 Show)))